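; BP_Door is a placeable door that configures an embedded interaction object, apparently for teleporting to another location.
; On BeginPlay it casts its child actor to BP_ObjecctInteraction_Door and passes it a Sequence, the Scene component's world location as the teleport target, and ToWhere as the interact widget's use text.
; The door holds only this setup, with no interaction or teleport logic in its own graphs.
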(event EventBeginPlay
  (bind _asbp_objecct_interaction_door (Utilities|Casting|CastToBP_ObjecctInteraction_Door (Variables|/Script/Engine.ChildActorComponent|GetChildActor (Variables|Default|GetBP_ObjecctInteraction_Door))))
  (Variables|/Game/BP_ObjecctInteraction_Door.BP_ObjecctInteraction_Door_C|SetSequence _asbp_objecct_interaction_door (Variables|Default|GetSequence))
  (Variables|/Game/BP_ObjecctInteraction_Door.BP_ObjecctInteraction_Door_C|SetTeleportHere _asbp_objecct_interaction_door (Transformation|GetWorldLocation (Variables|Default|GetScene)))
  (Variables|/Game/Gameplay/Blueprints/BP_InteractableObject.BP_InteractableObject_C|SetInteractWidgetUseText _asbp_objecct_interaction_door (Utilities|Text|ToText(String) (Variables|Default|GetTo%20Where?))))

(event Collision|EventActorBeginOverlap
  (params (OtherActor :type Actor%20Object%20Reference)))

(event EventTick
  (params (DeltaSeconds :type Float%20%28single-precision%29)))

(fn ConstructionScript)