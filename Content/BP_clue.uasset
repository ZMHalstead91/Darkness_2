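; Interactable book clue that shows a text clue on screen when a character uses it.
; On use, it passes its BookTextIndex to the shared W_BookClue widget held by BP_Darkness_GameInstance, then adds it to the viewport.
; A NotInUse flag blocks repeat use until leaving the trigger removes the widget and re-arms it.
; After use, it hides the player's interact message.
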(event EventBeginPlay)

(event Collision|EventActorBeginOverlap
  (params (OtherActor :type Actor%20Object%20Reference)))

(event EventPostObjectUsed
  (Class|BPIObjectInteraction|ToggleInteract(Message) (Game|GetPlayerCharacter 0) false 0.0))

(event EventTick
  (params (DeltaSeconds :type Float%20%28single-precision%29))
  (|CallParentFunction DeltaSeconds))

(event EventEndTriggerOverlap
  (params (Actor :type Actor%20Object%20Reference) (SideOptions :type Struct%20Interaction%20Options%20Structure) (Trigger :type Box%20Component%20Object%20Reference))
  (|CallParentFunction Actor SideOptions Trigger)
  (bind _asbp_darkness_game_instance (Utilities|Casting|CastToBP_Darkness_GameInstance (Game|GetGameInstance)))
  (bind _asw_book_clue (Utilities|Casting|CastToW_BookClue (Variables|/Game/Base/BP_Darkness_GameInstance.BP_Darkness_GameInstance_C|GetBookClue_Ref _asbp_darkness_game_instance)))
  (Widget|RemovefromParent _asw_book_clue)
  (Variables|Default|SetNotInUse true))

(fn ConstructionScript
  (|CallParentFunction))

(fn BeginUse
  (params (Character :type Character%20Object%20Reference) (InteractSide :type Struct%20Interaction%20Options%20Structure) (Trigger :type Box%20Component%20Object%20Reference))
  (bind _canuse_ (|CallParentFunction Character InteractSide Trigger))
  (if (Variables|Default|GetNotInUse)
    (Variables|Default|SetNotInUse false)
    (Variables|Default|SetGrace Character)
    (bind _asbp_darkness_game_instance (Utilities|Casting|CastToBP_Darkness_GameInstance (Game|GetGameInstance))
      (:then
        (bind _asw_book_clue (Utilities|Casting|CastToW_BookClue (Variables|/Game/Base/BP_Darkness_GameInstance.BP_Darkness_GameInstance_C|GetBookClue_Ref _asbp_darkness_game_instance))
          (:then
            (Default|SetText _asw_book_clue (Variables|Components|GetBookTextIndex))
            (Default|DisplayClue _asw_book_clue)
            (UserInterface|Viewport|AddtoViewport (Variables|/Game/Base/BP_Darkness_GameInstance.BP_Darkness_GameInstance_C|GetBookClue_Ref _asbp_darkness_game_instance) 0))
          (:CastFailed
            _)))
      (:CastFailed
        _))
    (return _canuse_)))