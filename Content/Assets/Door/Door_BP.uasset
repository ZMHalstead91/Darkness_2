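; Door actor that swings its mesh open and closes it when a Player-tagged actor leaves its Box while open.
; OpenDoor and CloseDoor use timelines as update loops, adding fixed rotation steps and setting Opened from yaw limits.
; OpenDoor has no active caller here; Open, CanUse? and ShouldAutoRemove? are stubs that do nothing or return false.
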(event OnComponentEndOverlap(Box)
  (params (OverlappedComponent :type Primitive%20Component%20Object%20Reference) (OtherActor :type Actor%20Object%20Reference) (OtherComp :type Primitive%20Component%20Object%20Reference) (OtherBodyIndex :type Integer))
  (if (and (Actor|ActorHasTag OtherActor "Player") (Variables|Default|GetOpened))
    (CallFunction|CloseDoor)))

(event Custom|OpenDoor
  (bind _model_door_josefrancisco__1_ (Variables|Default|GetModel_Door_JoseFrancisco__1_))
  (Timeline|Timeline_0 Play
    (:Update
      (if (Variables|Default|GetOpened)
        (Timeline|Timeline_0 Reverse)
        (else
          (Transformation|AddWorldRotation _model_door_josefrancisco__1_ "0,2.000000, 0" false false)
          (if (>= (.yaw (Variables|/Script/Engine.SceneComponent|GetRelativeRotation _model_door_josefrancisco__1_)) 9e+01)
            (Variables|Default|SetOpened true)
            (else
              (Variables|Default|SetOpened false))))))))

(event Custom|CloseDoor
  (bind _model_door_josefrancisco__1_ (Variables|Default|GetModel_Door_JoseFrancisco__1_))
  (Timeline|Timeline_1 Play
    (:Update
      (if (Variables|Default|GetOpened)
        (Transformation|AddWorldRotation _model_door_josefrancisco__1_ "0,-2.000000, 0" false false)
        (if (<= (.yaw (Variables|/Script/Engine.SceneComponent|GetRelativeRotation _model_door_josefrancisco__1_)) 0.0)
          (Variables|Default|SetOpened false)
          (else
            (Variables|Default|SetOpened true)))))))

(event EventBeginPlay)

(event Collision|EventActorBeginOverlap
  (params (OtherActor :type Actor%20Object%20Reference)))

(event EventTick
  (params (DeltaSeconds :type Float%20%28single-precision%29)))

(fn ConstructionScript)

(fn Open)

(fn CanUse?
  (params (UsingActor :type Actor%20Object%20Reference))
  (return false))

(fn ShouldAutoRemove?
  (return false))