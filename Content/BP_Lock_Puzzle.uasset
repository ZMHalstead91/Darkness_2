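; BP_Lock_Puzzle is an interactable code lock puzzle that disappears once solved.
; On begin play it resets the shared W_Lock widget from the game instance and passes it the level-one setting.
; Using it sends its code to that widget and shows it with UI-only input and a mouse cursor.
; Tick polls the widget's Unlocked flag, then plays a hint tune and destroys the actor.
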(event Custom|Show%20Mouse
  (params (On/Off :type Boolean))
  (Variables|/Script/Engine.PlayerController|SetbShowMouseCursor (Game|GetPlayerController 0) On/Off))

(event EventBeginPlay
  (bind _asbp_darkness_game_instance (Utilities|Casting|CastToBP_Darkness_GameInstance (Game|GetGameInstance)))
  (bind _asw_lock (Utilities|Casting|CastToW_Lock (Variables|/Game/Base/BP_Darkness_GameInstance.BP_Darkness_GameInstance_C|GetLock_ref _asbp_darkness_game_instance)))
  (Variables|/Game/Maps/Testing/W_Lock.W_Lock_C|SetUnlocked _asw_lock false)
  (Variables|/Game/Maps/Testing/W_Lock.W_Lock_C|SetLevelOne? _asw_lock (Variables|Default|GetLevelone?)))

(event Collision|EventActorBeginOverlap
  (params (OtherActor :type Actor%20Object%20Reference)))

(event EventTick
  (params (DeltaSeconds :type Float%20%28single-precision%29))
  (|CallParentFunction DeltaSeconds)
  (bind _asbp_darkness_game_instance (Utilities|Casting|CastToBP_Darkness_GameInstance (Game|GetGameInstance)))
  (bind _asw_lock (Utilities|Casting|CastToW_Lock (Variables|/Game/Base/BP_Darkness_GameInstance.BP_Darkness_GameInstance_C|GetLock_ref _asbp_darkness_game_instance)))
  (if (Variables|/Game/Maps/Testing/W_Lock.W_Lock_C|GetUnlocked _asw_lock)
    (Audio|PlaySound2D "/Game/Audio/Hint_Tune.Hint_Tune")
    (Actor|DestroyActor)))

(event EventPostObjectUsed
  (Class|BPIObjectInteraction|ToggleInteract(Message) (Game|GetPlayerCharacter 0) false 0.0))

(fn ConstructionScript
  (|CallParentFunction))

(fn BeginUse
  (params (Character :type Character%20Object%20Reference) (InteractSide :type Struct%20Interaction%20Options%20Structure) (Trigger :type Box%20Component%20Object%20Reference))
  (bind _returnvalue (Game|GetPlayerController 0))
  (bind _canuse_ (|CallParentFunction Character InteractSide Trigger))
  (bind _asbp_darkness_game_instance (Utilities|Casting|CastToBP_Darkness_GameInstance (Game|GetGameInstance))
    (:then
      (bind _asw_lock (Utilities|Casting|CastToW_Lock (Variables|/Game/Base/BP_Darkness_GameInstance.BP_Darkness_GameInstance_C|GetLock_ref _asbp_darkness_game_instance)))
      (Variables|/Game/Maps/Testing/W_Lock.W_Lock_C|SetCode _asw_lock (Variables|Default|GetCode))
      (UserInterface|Viewport|AddtoViewport (Variables|/Game/Base/BP_Darkness_GameInstance.BP_Darkness_GameInstance_C|GetLock_ref _asbp_darkness_game_instance) 0)
      (Input|SetInputModeUIOnly _returnvalue (Variables|/Game/Base/BP_Darkness_GameInstance.BP_Darkness_GameInstance_C|GetLock_ref _asbp_darkness_game_instance) "DoNotLock")
      (Variables|/Script/Engine.PlayerController|SetbShowMouseCursor _returnvalue true))
    (:CastFailed
      _))
  (return _canuse_))