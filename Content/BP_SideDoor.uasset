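; BP_SideDoor is a door actor that wraps a side-door interaction object as a child actor and configures it per instance.
; On BeginPlay it casts the child to BP_ObjecctInteraction_SideDoor and passes in its sequence and the Scene component's world location as the teleport destination.
; It also sets the child's EndLevel flag from DontEndLevel and its interact widget text from GoWhere.
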(event EventBeginPlay
  (bind _asbp_objecct_interaction_side_door (Utilities|Casting|CastToBP_ObjecctInteraction_SideDoor (Variables|/Script/Engine.ChildActorComponent|GetChildActor (Variables|Default|GetBP_ObjecctInteraction_SideDoor))))
  (Variables|/Game/BP_ObjecctInteraction_SideDoor.BP_ObjecctInteraction_SideDoor_C|SetSequence _asbp_objecct_interaction_side_door (Variables|Default|GetSequence))
  (Variables|/Game/BP_ObjecctInteraction_SideDoor.BP_ObjecctInteraction_SideDoor_C|SetTeleportHere _asbp_objecct_interaction_side_door (Transformation|GetWorldLocation (Variables|Default|GetScene)))
  (bind _asbp_objecct_interaction_side_door_2 (Utilities|Casting|CastToBP_ObjecctInteraction_SideDoor (Variables|/Script/Engine.ChildActorComponent|GetChildActor (Variables|Default|GetBP_ObjecctInteraction_SideDoor))))
  (Variables|/Game/BP_ObjecctInteraction_SideDoor.BP_ObjecctInteraction_SideDoor_C|SetEndLevel _asbp_objecct_interaction_side_door_2 (Variables|Default|GetDontEndLevel?))
  (Variables|/Game/Gameplay/Blueprints/BP_InteractableObject.BP_InteractableObject_C|SetInteractWidgetUseText _asbp_objecct_interaction_side_door_2 (Variables|Default|GetGo%20Where?)))

(event Collision|EventActorBeginOverlap
  (params (OtherActor :type Actor%20Object%20Reference)))

(event EventTick
  (params (DeltaSeconds :type Float%20%28single-precision%29)))

(fn ConstructionScript)