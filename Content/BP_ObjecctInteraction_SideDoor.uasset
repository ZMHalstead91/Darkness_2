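; Interactable side door that swings open on use and moves the player to another spot or level.
; BeginUse stores the character and runs a timeline that yaws the mesh open with a sound.
; PostObjectUsed plays a sequence, waits, teleports the player to TeleportHere, then reverses the sequence with a closing sound.
; If EndLevel is true the door swings shut; otherwise the game instance loads a hardcoded Level_1_3.
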(event Custom|OpenDoor
  (Utilities|Casting|CastToBP_Darkness_GameInstance (Game|GetGameInstance))
  (Audio|PlaySound2D "/Game/Audio/WWID_Door_Opening_SFX_01.WWID_Door_Opening_SFX_01" 1.0)
  (bind _dooropenratio (Timeline|DoorOpenAlpha Play)
    (:Update
      (Transformation|SetRelativeRotation (Variables|Character|GetMesh) (Math|Rotator|Lerp(Rotator) (Math|Rotator|MakeRotator 0.0 0.0 0.0) (Math|Rotator|MakeRotator 0.0 0.0 9e+01) _dooropenratio) false false))))

(event Custom|Teleport
  (bind _sequence (Variables|Default|GetSequence))
  (bind _sequenceplayer (Variables|/Script/LevelSequence.LevelSequenceActor|GetSequencePlayer _sequence))
  (Sequencer|Player|Play _sequenceplayer :!class /Script/MovieScene.MovieSceneSequencePlayer)
  (Utilities|FlowControl|Delay 2.0)
  (Class|BPIObjectInteraction|ToggleInteract(Message) (Variables|Default|GetCharacter) false 0.0)
  (Transformation|SetActorLocation (Game|GetPlayerCharacter 0) (Variables|Default|GetTeleportHere) false true)
  (Class|MovieSceneSequencePlayer|PlayReverse _sequenceplayer)
  (bind _asbp_darkness_game_instance (Utilities|Casting|CastToBP_Darkness_GameInstance (Game|GetGameInstance)))
  (Audio|PlaySound2D "/Game/Audio/WWID_Door_Closing_SFX_01.WWID_Door_Closing_SFX_01" 1.0)
  (if (Variables|Default|GetEndLevel)
    (bind _dooropenratio (Timeline|DoorOpenAlpha Reverse)
      (:Update
        (Transformation|SetRelativeRotation (Variables|Character|GetMesh) (Math|Rotator|Lerp(Rotator) (Math|Rotator|MakeRotator 0.0 0.0 0.0) (Math|Rotator|MakeRotator 0.0 0.0 9e+01) _dooropenratio) false false)))
    (else
      (bind _asbp_darkness_game_instance_2 (Utilities|Casting|CastToBP_Darkness_GameInstance (Game|GetGameInstance)))
      (Default|LoadLevel _asbp_darkness_game_instance_2 "Level_1_3" true))))

(event EventBeginPlay)

(event Collision|EventActorBeginOverlap
  (params (OtherActor :type Actor%20Object%20Reference)))

(event EventTick
  (params (DeltaSeconds :type Float%20%28single-precision%29))
  (|CallParentFunction DeltaSeconds))

(event EventPostObjectUsed
  (CallFunction|Teleport)
  (Class|BPIObjectInteraction|ToggleInteract(Message) (Variables|Default|GetInteractingPlayer) false 0.0))

(fn ConstructionScript
  (|CallParentFunction))

(fn BeginUse
  (params (Character :type Character%20Object%20Reference) (InteractSide :type Struct%20Interaction%20Options%20Structure) (Trigger :type Box%20Component%20Object%20Reference))
  (bind _canuse_ (|CallParentFunction Character InteractSide Trigger))
  (Variables|Default|SetCharacter Character)
  (CallFunction|OpenDoor)
  (return _canuse_))