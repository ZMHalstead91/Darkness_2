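; An interactable stair transition that teleports the player between areas behind a level sequence transition.
; BeginUse calls the parent, stores the character and fires Teleport, which plays the sequence and waits on a fixed delay.
; It then hides the interact message, ends use, moves the player to the Scene component's location and plays the sequence in reverse.
; A door-closing sound follows, scaled by the game instance's effects volume.
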(event Custom|Teleport
  (bind _sequence (Variables|Default|GetSequence))
  (bind _sequenceplayer (Variables|/Script/LevelSequence.LevelSequenceActor|GetSequencePlayer _sequence))
  (Sequencer|Player|Play _sequenceplayer :!class /Script/MovieScene.MovieSceneSequencePlayer)
  (Utilities|FlowControl|Delay 2.0)
  (Class|BPIObjectInteraction|ToggleInteract(Message) (Variables|Default|GetCharacter) false 0.0)
  (CallFunction|EndUse)
  (Transformation|SetActorLocation (Game|GetPlayerCharacter 0) (Transformation|GetWorldLocation (Variables|Default|GetScene)) false true)
  (Class|MovieSceneSequencePlayer|PlayReverse _sequenceplayer)
  (bind _asbp_darkness_game_instance (Utilities|Casting|CastToBP_Darkness_GameInstance (Game|GetGameInstance)))
  (Audio|PlaySound2D "/Game/Audio/WWID_Door_Closing_SFX_01.WWID_Door_Closing_SFX_01" (/ (Math|Conversions|ToFloat(Integer) (Variables|/Game/Base/BP_Darkness_GameInstance.BP_Darkness_GameInstance_C|GetEffectsVolume _asbp_darkness_game_instance)) 1e+01)))

(event EventBeginPlay)

(event Collision|EventActorBeginOverlap
  (params (OtherActor :type Actor%20Object%20Reference)))

(event EventTick
  (params (DeltaSeconds :type Float%20%28single-precision%29))
  (|CallParentFunction DeltaSeconds))

(fn ConstructionScript
  (|CallParentFunction))

(fn BeginUse
  (params (Character :type Character%20Object%20Reference) (InteractSide :type Struct%20Interaction%20Options%20Structure) (Trigger :type Box%20Component%20Object%20Reference))
  (bind _canuse_ (|CallParentFunction Character InteractSide Trigger))
  (Variables|Default|SetCharacter Character)
  (CallFunction|Teleport)
  (return _canuse_))