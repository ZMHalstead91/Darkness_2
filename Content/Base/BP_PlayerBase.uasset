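; Base player character for a side-scrolling game with crouch, jump, climbing, character switching and follow toggling.
; Each tick it highlights the usable object best aligned with its facing by dot product, showing a prompt or auto-using it.
; Used objects receive movement input and block jumping, with release governed by hold, auto-release and velocity rules.
; Otherwise, forward movement follows a spline or world X, locking Y when no spline exists.
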(event Custom|InteractParentPress
  (bind _pickups (Variables|Default|GetPickups))
  (bind _item (Utilities|Array|Get(acopy) _pickups))
  (Utilities|UseInteractionMacro
    (:Return%20Pressed
      (Utilities|IsValid _item
        (:Is%20Valid
          (Class|UsableThingInterface|Used(Message) _item))))))

(event Custom|SimulateInput
  (params (AxisValue :type Float%20%28single-precision%29))
  (CallFunction|ForwardMovement AxisValue))

(event Custom|InteractParentRelease
  (bind _pickups (Variables|Default|GetPickups))
  (bind _item (Utilities|Array|Get(acopy) _pickups))
  (Utilities|UseInteractionMacro) ; enters at Released
)

(event EventBeginPlay
  (Pawn|SpawnDefaultController))

(event Collision|EventActorEndOverlap
  (params (OtherActor :type Actor%20Object%20Reference))
  (if (Utilities|DoesObjectImplementInterface OtherActor "/Game/Gameplay/Blueprints/Interfaces/UsableThingInterface.UsableThingInterface_C")
    (Utilities|Array|RemoveItem (Variables|Default|GetPickups) OtherActor)))

(event Collision|EventActorBeginOverlap
  (params (OtherActor :type Actor%20Object%20Reference))
  (if (Utilities|DoesObjectImplementInterface OtherActor "/Game/Gameplay/Blueprints/Interfaces/UsableThingInterface.UsableThingInterface_C")
    (Utilities|Array|AddUnique (Variables|Default|GetPickups) OtherActor)
    (CallFunction|AddInteractUI)
    (Default|SetUseText (Variables|InteractionInterface|GetInteractionUI) "Pickup")))

(event EventTick
  (params (DeltaSeconds :type Float%20%28single-precision%29))
  (Variables|Default|SetDeltaTime DeltaSeconds)
  (CallFunction|UpdateHighlightInteraction)
  (if (and (Variables|Default|GetIsCrouched?) (not (AI|Components|NavMovement|IsCrouching (Variables|Character|GetCharacterMovement))))
    (Character|Crouch)))

(event EventAddUsableActor
  (params (User :type Struct%20Interactable%20Actor%20Structure))
  (Utilities|Array|AddUnique (Variables|Default|GetUsableObjects) User))

(event EventRemoveUsableActor
  (params (User :type Struct%20Interactable%20Actor%20Structure))
  (Utilities|Array|RemoveItem (Variables|Default|GetUsableObjects) User))

(event EventOnWalkingOffLedge
  (params (PreviousFloorImpactNormal :type Vector%20%28by%20ref%29) (PreviousFloorContactNormal :type Vector%20%28by%20ref%29) (PreviousLocation :type Vector%20%28by%20ref%29) (TimeDelta :type Float%20%28single-precision%29))
  (|CallParentFunction PreviousFloorImpactNormal PreviousFloorContactNormal PreviousLocation TimeDelta)
  (CallFunction|EndInteractState))

(event EventToggleInteract
  (params (bActive :type Boolean) (InputDelay :type Float%20%28single-precision%29))
  (if bActive
    (CallFunction|BeginInteractState)
    (else
      (|EndPushStateAndInputDelay InputDelay))))

(event EventOnStartCrouch
  (params (HalfHeightAdjust :type Float%20%28single-precision%29) (ScaledHalfHeightAdjust :type Float%20%28single-precision%29))
  (|CallParentFunction HalfHeightAdjust ScaledHalfHeightAdjust)
  (Variables|Default|SetIsCrouched? true))

(event Input|ActionEvents|InputActionCrouch
  (params (Key :type Key%20Structure :default "AnyKey"))
  ;[1 1 1] Input Action Crouch: Triggers when the crouch button is pressed and toggles the crouch state.
  (:Pressed
    (|CanCrouch?)
    (if (not (Variables|Default|GetbIsCrouched))
      (Character|Crouch)
      (else
        (Character|UnCrouch)
        (Variables|Default|SetIsCrouched? false)))))

(event Input|ActionEvents|InputActionInteraction
  (params (Key :type Key%20Structure :default "AnyKey"))
  (bind _pickups (Variables|Default|GetPickups))
  (bind _item (Utilities|Array|Get(acopy) _pickups))
  (:Pressed
    (Utilities|UseInteractionMacro :!label _label
      (:Return%20Pressed
        (Utilities|IsValid _item
          (:Is%20Valid
            (Class|UsableThingInterface|Used(Message) _item))))))
  (:Released
    (goto _label Released)))

(event Input|ActionEvents|InputActionFollowToggle
  (params (Key :type Key%20Structure :default "AnyKey"))
  (:Pressed
    (Class|BPICharacterSwitching|ToggleShouldFollow(Message) (Game|GetGameMode))))

(event Input|ActionEvents|InputActionJump
  (params (Key :type Key%20Structure :default "AnyKey"))
  ;[1 1 1] Input Action Jump: Triggers when the jump button is pressed. Player will jump if they're not already in the air.
  (:Pressed
    (Character|Jump))
  (:Released
    (Character|StopJumping)))

(event Input|ActionEvents|InputActionSwitchCharacter
  (params (Key :type Key%20Structure :default "AnyKey"))
  (:Pressed
    (Class|BPICharacterSwitching|SwitchCharacter(Message) (Game|GetGameMode))))

(event Input|AxisEvents|InputAxisClimb
  (params (AxisValue :type Float%20%28single-precision%29))
  (bind _usedinteractableobject (Variables|InteractionInterface|GetUsedInteractableObject)
    (:then
      (Default|MoveUp _usedinteractableobject AxisValue))
    (:else
      _))
  (if (Variables|Default|GetIsClimbing?)
    (Pawn|Input|AddMovementInput (Transformation|GetActorUpVector) AxisValue false)))

(event Input|AxisEvents|InputAxisMoveForward
  (params (AxisValue :type Float%20%28single-precision%29))
  (CallFunction|ForwardMovement AxisValue))

(fn ConstructionScript
  (|CallParentFunction))

(fn UpdateHighlightInteraction
  (bind _currentdots (LocalVariables|GetCurrentDots))
  (bind (_indexofmaxvalue _maxvalue) (Math|Float|MaxOfFloatArray _currentdots))
  (bind _shouldupdate (CallFunction|ShouldUpdateHighlightInteraction))
  (if _shouldupdate
    (for _array_element (Variables|Default|GetUsableObjects)
      (Utilities|Array|Add (LocalVariables|GetCurrentDots) (Math|Vector|DotProduct (Math|Vector|Normalize (- (Transformation|GetActorLocation (.InteractableActor (Utilities|Struct|BreakStruct_InteractableActor _array_element))) (Transformation|GetActorLocation))) (Transformation|GetActorForwardVector))))
    (if (>= _maxvalue (Variables|Default|GetInteractDotThreshold))
      (CallFunction|GetBestInteractHighlight _indexofmaxvalue)
      (else
        (Variables|InteractionInterface|SetHighlightedInteraction "" :!label _label)
        (CallFunction|RemoveInteractUI)))
    (else
      (goto _label))))

(fn ShouldUpdateHighlightInteraction
  (bind _charactermovement (Variables|Character|GetCharacterMovement))
  (return (Math|Boolean|ANDBoolean (> (Utilities|Array|Length (Variables|Default|GetUsableObjects)) 0) (not (Utilities|IsValid (Variables|InteractionInterface|GetUsedInteractableObject))) (not (AI|Components|NavMovement|IsFalling _charactermovement)) (not (AI|Components|NavMovement|IsCrouching _charactermovement)) (not (Class|NavMovementComponent|IsFlying _charactermovement)))))

(fn CanStopUsingObject
  (params (InteractableObject :type BP%20Interactable%20Object%20Object%20Reference) (bHoldToInteractCheck :type Boolean))
  (bind _returnvalue (Transformation|GetVelocity InteractableObject))
  (bind (_x _y) (Math|Vector|BreakVector _returnvalue))
  (return (Math|Boolean|ANDBoolean (select bHoldToInteractCheck (Variables|/Game/Gameplay/Blueprints/BP_InteractableObject.BP_InteractableObject_C|GetbHoldToInteract InteractableObject) true) (not (Variables|/Game/Gameplay/Blueprints/BP_InteractableObject.BP_InteractableObject_C|GetbAutoRelease InteractableObject)) (select (not (Variables|/Game/Gameplay/Blueprints/BP_InteractableObject.BP_InteractableObject_C|GetbCanReleaseInMovement InteractableObject)) (Math|Float|NearlyEqual(Float) (Math|Vector|VectorLength (Math|Vector|MakeVector _x _y 0.0)) 0.0 1.0) true))))

(fn GetBestInteractHighlight
  (params (Index :type Integer))
  (bind _usableobjects (Variables|Default|GetUsableObjects))
  (bind _item (Utilities|Array|Get(acopy) _usableobjects Index))
  (bind _interactableactor (Utilities|Struct|BreakStruct_InteractableActor _item))
  (bind _interactableactor_2 (Utilities|Struct|BreakStruct_InteractableActor _item))
  (if (and (!= (.InteractableActor (Utilities|Struct|BreakStruct_InteractableActor (Variables|InteractionInterface|GetHighlightedInteraction))) _interactableactor) (not (Utilities|IsValid (Variables|/Game/Gameplay/Blueprints/BP_InteractableObject.BP_InteractableObject_C|GetInteractingPlayer _interactableactor))))
    (Variables|InteractionInterface|SetHighlightedInteraction _item)
    (Utilities|IsValid _interactableactor_2
      (:Is%20Valid
        (if (Variables|/Game/Gameplay/Blueprints/BP_InteractableObject.BP_InteractableObject_C|GetbAutoUse _interactableactor_2)
          (if (not (Variables|/Game/Gameplay/Blueprints/BP_InteractableObject.BP_InteractableObject_C|GetbAutoRelease _interactableactor_2))
            (CallFunction|AddInteractUI))
          (CallFunction|BeginInteractState)
          (Utilities|Array|RemoveItem (Variables|Default|GetUsableObjects) (Variables|InteractionInterface|GetHighlightedInteraction))
          (else
            (CallFunction|AddInteractUI)))))))

(fn RemoveInteractUI
  (Utilities|IsValid (Variables|InteractionInterface|GetUsedInteractableObject)
    (:Is%20Not%20Valid
      (if (<= (Utilities|Array|Length (Variables|Default|GetPickups)) 0)
        (bind _interactionui (Variables|InteractionInterface|GetInteractionUI)
          (:then
            (if (Widget|IsVisible _interactionui)
              (Widget|RemovefromParent _interactionui)))
          (:else))))))

(fn AddInteractUI
  (bind _highlightedinteraction (Variables|InteractionInterface|GetHighlightedInteraction))
  (bind _interactableactor (Utilities|Struct|BreakStruct_InteractableActor _highlightedinteraction))
  (bind _interactionui (Variables|InteractionInterface|GetInteractionUI)
    (:then
      (if (not (Widget|IsVisible _interactionui))
        (UserInterface|Viewport|AddtoViewport _interactionui 0)
        (Utilities|IsValid _interactableactor :!label _label
          (:Is%20Valid
            (Default|SetUseText (Variables|InteractionInterface|GetInteractionUI) (Variables|/Game/Gameplay/Blueprints/BP_InteractableObject.BP_InteractableObject_C|GetInteractWidgetUseText _interactableactor))))))
    (:else
      (bind _returnvalue (UserInterface|CreateWidget "/Game/UI/W_PushInteract.W_PushInteract_C" (Game|GetPlayerController 0)))
      (bind _output_get (Variables|InteractionInterface|SetInteractionUI _returnvalue))
      (UserInterface|Viewport|AddtoViewport _output_get 0)
      (goto _label))))

(fn BeginInteractState
  (bind _highlightedinteraction (Variables|InteractionInterface|GetHighlightedInteraction))
  (bind (_interactableactor _interactsideoptions _interactionside) (Utilities|Struct|BreakStruct_InteractableActor _highlightedinteraction))
  (Utilities|IsValid _interactableactor
    (:Is%20Valid
      (bind _output_get (Variables|InteractionInterface|SetUsedInteractableObject _interactableactor))
      (bind _canuse_ (Default|BeginUse _output_get self _interactsideoptions _interactionside))
      (bind _interactionui (Variables|InteractionInterface|GetInteractionUI)
        (:then
          (Default|ToggleGrabbed _interactionui _canuse_)
          (if (Variables|/Game/Gameplay/Blueprints/BP_InteractableObject.BP_InteractableObject_C|GetOneShot? _output_get)
            (CallFunction|RemoveUsableActor (Variables|InteractionInterface|GetHighlightedInteraction))
            (Widget|RemovefromParent (Variables|InteractionInterface|GetInteractionUI)))
          (Default|PostObjectUsed _output_get))
        (:else)))))

(fn EndInteractState
  (bind _usedinteractableobject (Variables|InteractionInterface|GetUsedInteractableObject)
    (:then
      (Default|EndUse _usedinteractableobject))
    (:else
      _))
  (bind _interactionui (Variables|InteractionInterface|GetInteractionUI)
    (:then
      (Default|ToggleGrabbed _interactionui false))
    (:else
      _))
  (Variables|InteractionInterface|SetUsedInteractableObject 0))

(fn CanJumpInternal
  (bind _returnvalue (|CallParentFunction))
  (return (Math|Boolean|ANDBoolean _returnvalue (not (Utilities|IsValid (Variables|InteractionInterface|GetUsedInteractableObject))) (not (AI|Components|NavMovement|IsCrouching (Variables|Character|GetCharacterMovement))) (not (Variables|Default|GetIsClimbing?)))))

(fn ForwardMovement
  (params (InputPin :type Float%20%28single-precision%29))
  (bind _returnvalue (Transformation|GetActorLocation))
  (bind _usedinteractableobject (Variables|InteractionInterface|GetUsedInteractableObject)
    (:then
      (Default|MoveForward _usedinteractableobject InputPin))
    (:else
      (if (or (not (Variables|Default|GetIsClimbing?)) (Variables|Default|GetFollowing?))
        (Utilities|IsValid (Variables|/Game/Gameplay/Blueprints/Components/SplinePathing.SplinePathing_C|GetSplineToFollow (Variables|Default|GetSplinePathing))
          (:Is%20Valid
            (bind _extentreached_ (Default|AddInput (Variables|Default|GetSplinePathing) InputPin (Class|MovementComponent|GetMaxSpeed (Variables|Character|GetCharacterMovement))))
            (if (not _extentreached_)
              (Pawn|Input|AddMovementInput "1.000000, 0, 0" InputPin false :!label _label)))
          (:Is%20Not%20Valid
            (Transformation|SetActorLocation (Math|Vector|MakeVector (.x _returnvalue) 84.0 (.z _returnvalue)) true false)
            (goto _label)))))))