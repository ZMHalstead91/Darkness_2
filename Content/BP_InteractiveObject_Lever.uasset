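; Interactive lever that the player flips back and forth between two positions.
; The BeginUse override calls its parent, then LeverPull, which plays a pull sound and uses a FlipFlop to alternately set or clear the Toggle flag.
; Each flip plays or reverses the LevelPullAlpha timeline, which lerps the mesh's relative pitch between the two angles.
; PostObjectUsed hides the player's interact message.
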(event Custom|LeverPull
  (Audio|PlaySound2D "/Game/Audio/Lever_Pull.Lever_Pull")
  (Utilities|FlowControl|FlipFlop
    (:A
      (Variables|Default|SetToggle true)
      (bind _lerp (Timeline|LevelPullAlpha PlayFromStart)
        (:Update
          (Transformation|SetRelativeRotation (Variables|Character|GetMesh) (Math|Rotator|Lerp(Rotator) (Math|Rotator|MakeRotator 0.0 25.0 0.0) (Math|Rotator|MakeRotator 0.0 -25.0 0.0) _lerp) false false))))
    (:B
      (Variables|Default|SetToggle false)
      (Timeline|LevelPullAlpha ReverseFromEnd))))

(event EventBeginPlay)

(event Collision|EventActorBeginOverlap
  (params (OtherActor :type Actor%20Object%20Reference)))

(event EventPostObjectUsed
  (Class|BPIObjectInteraction|ToggleInteract(Message) (Game|GetPlayerCharacter 0) false 0.0))

(event EventTick
  (params (DeltaSeconds :type Float%20%28single-precision%29))
  (|CallParentFunction DeltaSeconds))

(fn ConstructionScript
  (|CallParentFunction))

(fn BeginUse
  (params (Character :type Character%20Object%20Reference) (InteractSide :type Struct%20Interaction%20Options%20Structure) (Trigger :type Box%20Component%20Object%20Reference))
  (bind _canuse_ (|CallParentFunction Character InteractSide Trigger))
  (CallFunction|LeverPull)
  (return _canuse_))