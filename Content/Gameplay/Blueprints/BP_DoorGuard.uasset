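; BP_DoorGuard is a guard NPC that turns the player back until every item in MatchingItemIds has been picked up.
; ItemPickedUp removes matching IDs from that list.
; While IDs remain, player overlap disables input, plays a voice line, subtitle widget and montage, then walks the player to PushbackPoint via SimpleMoveToLocation before restoring input.
; Once the list is empty, overlap plays a different line once, without pushback.
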(event Custom|TurnOffDialouge
  (params (Time :type Float%20%28single-precision%29))
  (Utilities|FlowControl|Delay Time)
  (Widget|RemovefromParent (Variables|Default|GetDialouge)))

(event EventBeginPlay)

(event Collision|EventActorBeginOverlap
  (params (OtherActor :type Actor%20Object%20Reference))
  (bind _ascharacter (Utilities|Casting|CastToCharacter OtherActor))
  (if (Actor|ActorHasTag OtherActor "Player")
    (if (> (Utilities|Array|Length (Variables|Default|GetMatchingItemIds)) 0)
      (Input|DisableInput _ascharacter 0)
      (Audio|PlaySound2D "/Game/Audio/Dialogue/Foreman/DIAL_FM_BackToWork_01.DIAL_FM_BackToWork_01")
      (bind _returnvalue (UserInterface|CreateWidget "/Game/UI/W_Dialouge.W_Dialouge_C"))
      (bind _output_get (Variables|Default|SetDialouge _returnvalue))
      (Default|Line4 _output_get)
      (UserInterface|Viewport|AddtoViewport _returnvalue 0)
      (CallFunction|TurnOffDialouge 3.0)
      (Animation|PlayAnimMontage "/Game/Assets/MaleNPC/Anims/MaleNPC_Conversation_HandsOnOveralls_Montage.MaleNPC_Conversation_HandsOnOveralls_Montage" 1.0 "Default")
      (Utilities|FlowControl|Delay 1.0)
      (AI|Navigation|SimpleMovetoLocation (Game|GetPlayerController 0) (.location (Transformation|GetWorldTransform (Variables|Default|GetPushbackPoint))))
      (Utilities|FlowControl|Delay 1.25)
      (Input|EnableInput _ascharacter 0)
      (else
        (Utilities|FlowControl|DoOnce false
          (:Completed
            (Audio|PlaySound2D "/Game/Audio/Dialogue/Grace/Grace_L11.Grace_L11")
            (bind _returnvalue_2 (UserInterface|CreateWidget "/Game/UI/W_Dialouge.W_Dialouge_C"))
            (bind _output_get_2 (Variables|Default|SetDialouge _returnvalue_2))
            (Default|Line5 _output_get_2)
            (UserInterface|Viewport|AddtoViewport _returnvalue_2 0)
            (CallFunction|TurnOffDialouge 4.0)))))))

(event EventTick
  (params (DeltaSeconds :type Float%20%28single-precision%29)))

(event EventItemPickedUp
  (params (ItemID :type String))
  (bind _matchingitemids (Variables|Default|GetMatchingItemIds))
  (bind _returnvalue (Utilities|Array|FindItem _matchingitemids ItemID))
  (if (!= _returnvalue -1)
    (Utilities|Array|RemoveIndex _matchingitemids _returnvalue)
    (if (<= (Utilities|Array|Length (Variables|Default|GetMatchingItemIds)) 0)
      _)))

(fn ConstructionScript)