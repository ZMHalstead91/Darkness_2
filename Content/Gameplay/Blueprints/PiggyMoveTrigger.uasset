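; PiggyMoveTrigger is a trigger actor that sends a set of pigs moving when a bucket enters it.
; The first overlap of its Trigger component by a BP_Bucket calls MakePigsMove, which calls MoveToEvent on every entry in PiggiesToNotify.
; Both the overlap and MakePigsMove are gated by DoOnce, so the pigs are notified only once.
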(event OnComponentBeginOverlap(Trigger)
  (params (OverlappedComponent :type Primitive%20Component%20Object%20Reference) (OtherActor :type Actor%20Object%20Reference) (OtherComp :type Primitive%20Component%20Object%20Reference) (OtherBodyIndex :type Integer) (bFromSweep :type Boolean) (SweepResult :type Hit%20Result%20Structure%20%28by%20ref%29))
  (Utilities|Casting|CastToBP_Bucket OtherActor)
  (Utilities|FlowControl|DoOnce false
    (:Completed
      (CallFunction|MakePigsMove))))

(event Custom|MakePigsMove
  (Utilities|FlowControl|DoOnce false
    (:Completed
      (for _array_element (Variables|Default|GetPiggiesToNotify)
        (Default|MovetoEvent _array_element)))))

(event EventBeginPlay)

(event EventTick
  (params (DeltaSeconds :type Float%20%28single-precision%29)))

(fn ConstructionScript
  (|CallParentFunction))