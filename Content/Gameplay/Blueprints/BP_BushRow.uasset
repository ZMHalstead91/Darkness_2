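; BP_BushRow is a placeable actor that lays out a straight row of bush instances at construction time, with no active event logic.
; The construction script sizes the BushArea box from configurable extents and derives the bush count from its scaled X extent and the spacing distance.
; It adds instances to BushInstances in both directions along the box's forward vector, plus one at BushesOrigin, all sharing the origin's rotation.
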(event EventBeginPlay)

(event Collision|EventActorBeginOverlap
  (params (OtherActor :type Actor%20Object%20Reference)))

(event EventTick
  (params (DeltaSeconds :type Float%20%28single-precision%29)))

(fn ConstructionScript
  (bind _busharea (Variables|Default|GetBushArea))
  (bind _bushspreaddist (Variables|Default|GetBushSpreadDist))
  (bind _bushspreaddist_2 (Variables|Default|GetBushSpreadDist))
  (bind _bushesorigin (Variables|Default|GetBushesOrigin))
  (bind _bushesorigin_2 (Variables|Default|GetBushesOrigin))
  (bind _bushspreaddist_3 (Variables|Default|GetBushSpreadDist))
  (bind _returnvalue (Components|Box|GetScaledBoxExtent _busharea))
  (bind _returnvalue_2 (/ (.x _returnvalue) _bushspreaddist_3))
  (bind _returnvalue_3 (Math|Float|Truncate _returnvalue_2))
  (bind _returnvalue_4 (- _returnvalue_3 1))
  (Components|Box|SetBoxExtent (Variables|Default|GetBushArea) (Variables|Default|GetBushRowBoxExtents) true)
  (for _index (range 0 _returnvalue_4)
    (Class|InstancedStaticMeshComponent|AddInstanceWorldSpace (Variables|Default|GetBushInstances) (Math|Transform|MakeTransform (+ (* (Math|Vector|NegateVector (Math|Vector|GetForwardVector (Variables|Default|GetBushArea))) (+ _bushspreaddist (* _index _bushspreaddist))) (Transformation|GetWorldLocation _bushesorigin)) (Transformation|GetWorldRotation _bushesorigin))))
  (for _index_2 (range 0 _returnvalue_4)
    (Class|InstancedStaticMeshComponent|AddInstanceWorldSpace (Variables|Default|GetBushInstances) (Math|Transform|MakeTransform (+ (Transformation|GetWorldLocation _bushesorigin_2) (* (Math|Vector|GetForwardVector (Variables|Default|GetBushArea)) (+ _bushspreaddist_2 (* _index_2 _bushspreaddist_2)))) (Transformation|GetWorldRotation _bushesorigin_2))))
  (Class|InstancedStaticMeshComponent|AddInstanceWorldSpace (Variables|Default|GetBushInstances) (Transformation|GetWorldTransform _bushesorigin_2)))