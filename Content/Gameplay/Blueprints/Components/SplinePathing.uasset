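; Actor component that moves its owner along a spline path from axis input, keeping the owner's own Z height.
; AddInput advances a clamped target distance and reports when it hits either end; SetNewSplineToFollow switches paths at a given distance.
; Tick sweeps the owner to the current distance, committing the target only if that succeeds, and turns the capsule along the spline, flipped for negative input.
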(event EventBeginPlay
  (Variables|Default|SetOwnerCapsule_Ref (Actor|GetComponentbyClass (Components|GetOwner) "/Script/Engine.CapsuleComponent")))

(event EventTick
  (params (DeltaSeconds :type Float%20%28single-precision%29))
  (Utilities|IsValid (Variables|Default|GetSplineToFollow)
    (:Is%20Valid
      (bind _output_get (Variables|Default|SetCharacterLocation (Math|Vector|MakeVector (.x (Spline|GetLocationatDistanceAlongSpline (Variables|/Game/Gameplay/Blueprints/BP_SplinePath.BP_SplinePath_C|GetPath (Variables|Default|GetSplineToFollow)) (Variables|Default|GetSplineDistance) "World")) (.y (Spline|GetLocationatDistanceAlongSpline (Variables|/Game/Gameplay/Blueprints/BP_SplinePath.BP_SplinePath_C|GetPath (Variables|Default|GetSplineToFollow)) (Variables|Default|GetSplineDistance) "World")) (.z (Transformation|GetActorLocation (Components|GetOwner))))))
      (bind _returnvalue (Transformation|SetActorLocation (Components|GetOwner) _output_get true false))
      (if _returnvalue
        (Variables|Default|SetSplineDistance (Variables|Default|GetNewSplineDistance)))
      (Variables|Default|SetCurrentRotation (Spline|GetRotationatDistanceAlongSpline (Variables|/Game/Gameplay/Blueprints/BP_SplinePath.BP_SplinePath_C|GetPath (Variables|Default|GetSplineToFollow)) (Variables|Default|GetSplineDistance) "World"))
      (Utilities|IsValid (Variables|Default|GetOwnerCapsule_Ref)
        (:Is%20Valid
          (Math|Float|CompareFloat (Variables|Default|GetMovementInput) 0.0
            (:>
              (Transformation|SetWorldRotation (Variables|Default|GetOwnerCapsule_Ref) (Variables|Default|GetCurrentRotation) false false))
            (:<
              (Transformation|SetWorldRotation (Variables|Default|GetOwnerCapsule_Ref) (Math|Rotator|CombineRotators (Variables|Default|GetCurrentRotation) "0,-180.000000, 0") false false))))))))

(fn AddInput
  (params (AxisInput :type Float%20%28single-precision%29) (MaxSpeed :type Float%20%28single-precision%29))
  (bind _splinetofollow (Variables|Default|GetSplineToFollow))
  (bind _path (Variables|/Game/Gameplay/Blueprints/BP_SplinePath.BP_SplinePath_C|GetPath _splinetofollow))
  (bind _returnvalue (Spline|GetSplineLength _path))
  (Variables|Default|SetMovementInput AxisInput)
  (bind _output_get (LocalVariables|SetMoveAmount (* (Variables|Default|GetMovementInput) MaxSpeed (Utilities|Time|GetWorldDeltaSeconds))))
  (bind _output_get_2 (Variables|Default|SetNewSplineDistance (Math|Float|Clamp(Float) (+ _output_get (Variables|Default|GetSplineDistance)) 0.0 _returnvalue)))
  (return (or (<= _output_get_2 0.0) (>= _output_get_2 _returnvalue))))

(fn SetNewSplinetoFollow
  (params (NewPath :type BP%20Spline%20Path%20Object%20Reference) (DistAlongSpline :type Float%20%28single-precision%29))
  (if (!= NewPath (Variables|Default|GetSplineToFollow))
    (Variables|Default|SetSplineToFollow NewPath)
    (Variables|Default|SetSplineDistance DistAlongSpline)
    (Variables|Default|SetNewSplineDistance DistAlongSpline)))