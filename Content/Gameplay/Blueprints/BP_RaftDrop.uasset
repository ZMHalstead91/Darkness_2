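; BP_RaftDrop is an actor that releases a bucket when its lever is used, with a rope-snap effect.
; On BeginPlay it casts its lever child actor to BP_InteractiveObject_Lever and binds MovePlatform to the lever's use-started event.
; MovePlatform destroys the static mesh component, plays a 2D rope-snap sound, then calls ApplyPhysics on the BP_Bucket child actor.
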(event Custom|Move%20Platform
  (Components|DestroyComponent (Variables|Default|GetStaticMesh))
  (Audio|PlaySound2D "/Game/Audio/Rope_Snap.Rope_Snap")
  (bind _asbp_bucket (Utilities|Casting|CastToBP_Bucket (Variables|/Script/Engine.ChildActorComponent|GetChildActor (Variables|Default|GetBP_Bucket))))
  (Default|ApplyPhysics _asbp_bucket))

(event EventBeginPlay
  (bind _asbp_interactive_object_lever (Utilities|Casting|CastToBP_InteractiveObject_Lever (Variables|/Script/Engine.ChildActorComponent|GetChildActor (Variables|Default|GetBP_InteractiveObject_Lever))))
  (EventDispatchers|BindEventtoUseStarted _asbp_interactive_object_lever (delegate Custom|Move%20Platform)))

(event Collision|EventActorBeginOverlap
  (params (OtherActor :type Actor%20Object%20Reference)))

(event EventTick
  (params (DeltaSeconds :type Float%20%28single-precision%29)))

(fn ConstructionScript)