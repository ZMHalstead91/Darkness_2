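; Interactable fence that characters crawl under, usable only by actors implementing Crawling_Interface.
; Trigger overlaps are forwarded to the parent only for such actors, and BeginUse either starts the crawl or sends an unable-to-use message.
; After a short delay, the crawl disables mesh collision, messages the character to crawl, then restores collision once the character's current montage length has elapsed.
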(event Custom|SendCrawlMessage
  (params (Character :type Character%20Object%20Reference))
  (Utilities|FlowControl|Delay 1.0)
  (Collision|SetCollisionEnabled (Variables|Default|GetMeshCollision) "NoCollision")
  (Class|CrawlingInterface|BeginCrawling(Message) Character)
  (bind _returnvalue (Animation|GetCurrentMontage Character :!class /Script/Engine.Character))
  (bind _returnvalue_2 (Animation|GetPlayLength _returnvalue))
  (Utilities|FlowControl|Delay _returnvalue_2)
  (Collision|SetCollisionEnabled (Variables|Default|GetMeshCollision) "QueryAndPhysics"))

(event EventBeginTriggerOverlap
  (params (Actor :type Actor%20Object%20Reference) (SideOptions :type Struct%20Interaction%20Options%20Structure) (Trigger :type Box%20Component%20Object%20Reference))
  (if (Utilities|DoesObjectImplementInterface Actor "/Game/Gameplay/Blueprints/Interfaces/Crawling_Interface.Crawling_Interface_C")
    (|CallParentFunction Actor SideOptions Trigger)))

(event EventEndTriggerOverlap
  (params (Actor :type Actor%20Object%20Reference) (SideOptions :type Struct%20Interaction%20Options%20Structure) (Trigger :type Box%20Component%20Object%20Reference))
  (if (Utilities|DoesObjectImplementInterface Actor "/Game/Gameplay/Blueprints/Interfaces/Crawling_Interface.Crawling_Interface_C")
    (|CallParentFunction Actor SideOptions Trigger)))

(event EventEndUse
  (|CallParentFunction))

(fn ConstructionScript
  (|CallParentFunction))

(fn BeginUse
  (params (Character :type Character%20Object%20Reference) (InteractSide :type Struct%20Interaction%20Options%20Structure) (Trigger :type Box%20Component%20Object%20Reference))
  (bind _canuse_ (|CallParentFunction Character InteractSide Trigger))
  (bind _output_get (LocalVariables|SetCanUseReturn (and _canuse_ (Utilities|DoesObjectImplementInterface Character "/Game/Gameplay/Blueprints/Interfaces/Crawling_Interface.Crawling_Interface_C"))))
  (if _output_get
    (CallFunction|SendCrawlMessage Character)
    (else
      (Class|BPIObjectInteraction|UnabletoUseItem(Message) Character)))
  (return (LocalVariables|GetCanUseReturn)))