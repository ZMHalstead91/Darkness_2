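; BP_Piggy is a pig character that walks to a preset spot and starts eating.
; On BeginPlay it stores the world location of its MoveToLocation component as the target.
; MoveToEvent runs AI MoveTo toward that target and, on success, sets IsEating on the mesh's AnimBP_Pig animation instance.
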(event Custom|MoveToEvent
  (AI|AIMoveTo self (Variables|Default|GetTargetLocation) 0 75.0 true
    (:OnSuccess
      (bind _asanim_bp_pig (Utilities|Casting|CastToAnimBP_Pig (Components|SkeletalMesh|GetAnimInstance (Variables|Character|GetMesh))))
      (Variables|/Game/Assets/Pig/Anims/AnimBP_Pig.AnimBP_Pig_C|SetIsEating? _asanim_bp_pig true))))

(event EventBeginPlay
  (Variables|Default|SetTargetLocation (Transformation|GetWorldLocation (Variables|Default|GetMoveToLocation))))

(event Collision|EventActorBeginOverlap
  (params (OtherActor :type Actor%20Object%20Reference)))

(event EventTick
  (params (DeltaSeconds :type Float%20%28single-precision%29)))

(fn ConstructionScript)