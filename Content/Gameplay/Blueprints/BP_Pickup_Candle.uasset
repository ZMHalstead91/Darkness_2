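; BP_Pickup_Candle is a candle pickup that, when used, checks off a quest log item and destroys itself.
; On BeginPlay it caches every actor implementing ItemPickupInterface.
; Used sends each listener the ObjectID, and inside that same loop updates W_Questlog through the game instance and plays a hint tune, so both repeat per listener.
; CanUse? and ShouldAutoRemove? both return false.
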(event EventBeginPlay
  (bind _outactors (Actor|GetAllActorswithInterface "/Game/Gameplay/Blueprints/Interfaces/ItemPickupInterface.ItemPickupInterface_C"))
  (Variables|Default|SetPickupListeners _outactors))

(event Collision|EventActorBeginOverlap
  (params (OtherActor :type Actor%20Object%20Reference)))

(event EventTick
  (params (DeltaSeconds :type Float%20%28single-precision%29)))

(event EventUsed
  (params (UsingActor :type Actor%20Object%20Reference) (Value :type Integer))
  (for _array_element (Variables|Default|GetPickupListeners)
    (Class|ItemPickupInterface|ItemPickedUp(Message) _array_element (Variables|Default|GetObjectID))
    (bind _asbp_darkness_game_instance (Utilities|Casting|CastToBP_Darkness_GameInstance (Game|GetGameInstance)))
    (bind _asw_questlog (Utilities|Casting|CastToW_Questlog (Variables|/Game/Base/BP_Darkness_GameInstance.BP_Darkness_GameInstance_C|GetQuestlog_Ref _asbp_darkness_game_instance)))
    (Default|CheckItem2 _asw_questlog true)
    (Audio|PlaySound2D "/Game/Audio/Hint_Tune.Hint_Tune"))
  (Actor|DestroyActor))

(fn ConstructionScript)

(fn CanUse?
  (params (UsingActor :type Actor%20Object%20Reference))
  (return false))

(fn ShouldAutoRemove?
  (return false))