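; Interactable object for the bottom of a ladder, which characters implementing Climbing_Interface use to start climbing.
; Trigger begin and end overlaps pass to the parent only for actors with that interface.
; BeginUse requires parent approval and the interface, then sends the mount-bottom message to the character after a one-second delay, or an unable-to-use message on failure.
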(event Custom|SendClimbMessage
  (params (ToCharacter :type Character%20Object%20Reference))
  (Utilities|FlowControl|Delay 1.0)
  (Class|ClimbingInterface|MountLadderBottom(Message) ToCharacter))

(event EventBeginPlay)

(event Collision|EventActorBeginOverlap
  (params (OtherActor :type Actor%20Object%20Reference)))

(event EventTick
  (params (DeltaSeconds :type Float%20%28single-precision%29))
  (|CallParentFunction DeltaSeconds))

(event EventBeginTriggerOverlap
  (params (Actor :type Actor%20Object%20Reference) (SideOptions :type Struct%20Interaction%20Options%20Structure) (Trigger :type Box%20Component%20Object%20Reference))
  (if (Utilities|DoesObjectImplementInterface Actor "/Game/Gameplay/Blueprints/Interfaces/Climbing_Interface.Climbing_Interface_C")
    (|CallParentFunction Actor SideOptions Trigger)))

(event EventEndTriggerOverlap
  (params (Actor :type Actor%20Object%20Reference) (SideOptions :type Struct%20Interaction%20Options%20Structure) (Trigger :type Box%20Component%20Object%20Reference))
  (if (Utilities|DoesObjectImplementInterface Actor "/Game/Gameplay/Blueprints/Interfaces/Climbing_Interface.Climbing_Interface_C")
    (|CallParentFunction Actor SideOptions Trigger)))

(fn ConstructionScript
  (|CallParentFunction))

(fn BeginUse
  (params (Character :type Character%20Object%20Reference) (InteractSide :type Struct%20Interaction%20Options%20Structure) (Trigger :type Box%20Component%20Object%20Reference))
  (bind _canuse_ (|CallParentFunction Character InteractSide Trigger))
  (bind _output_get (LocalVariables|SetCanUseReturn (and _canuse_ (Utilities|DoesObjectImplementInterface Character "/Game/Gameplay/Blueprints/Interfaces/Climbing_Interface.Climbing_Interface_C"))))
  (if _output_get
    (CallFunction|SendClimbMessage Character)
    (else
      (Class|BPIObjectInteraction|UnabletoUseItem(Message) Character)))
  (return (LocalVariables|GetCanUseReturn)))