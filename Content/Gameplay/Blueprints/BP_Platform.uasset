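; BP_Platform is a lifting platform actor that raises and lowers its PlatformModel between its base position and a height set by GOUP.
; A timeline, PlatformLifting, drives a lerped relative transform on the model, played forward to rise and reversed to descend.
; LiftUP and LiftDown functions wrap the GoUp and GoDown events so the lift can be triggered from outside.
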(event Custom|GoUp
  (bind _lerp (Timeline|PlatformLifting Play)
    (:Update
      (Transformation|SetRelativeTransform (Variables|Default|GetPlatformModel) (Math|Transform|Lerp(Transform) (Math|Transform|MakeTransform "0, 0, 0" "0.000000, 0, 0") (Math|Transform|MakeTransform (Math|Vector|MakeVector 0.0 0.0 (Variables|Default|GetGO%20UP)) "0.000000, 0, 0") _lerp) false false))))

(event Custom|GoDown
  (bind _lerp (Timeline|PlatformLifting Reverse)
    (:Update
      (Transformation|SetRelativeTransform (Variables|Default|GetPlatformModel) (Math|Transform|Lerp(Transform) (Math|Transform|MakeTransform "0, 0, 0" "0.000000, 0, 0") (Math|Transform|MakeTransform (Math|Vector|MakeVector 0.0 0.0 (Variables|Default|GetGO%20UP)) "0.000000, 0, 0") _lerp) false false))))

(event EventBeginPlay)

(event Collision|EventActorBeginOverlap
  (params (OtherActor :type Actor%20Object%20Reference)))

(event EventTick
  (params (DeltaSeconds :type Float%20%28single-precision%29)))

(fn ConstructionScript)

(fn LiftUP
  (CallFunction|GoUp))

(fn LiftDown
  (CallFunction|GoDown))