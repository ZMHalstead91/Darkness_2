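; BP_ConversationActor is a character actor meant for conversations, with an early placeholder for the dialogue itself.
; The construction script applies its CharacterMesh and AnimInstance variables to the skeletal mesh.
; On BeginPlay it casts the ConversationInteraction child actor to BP_InteractableObject and binds a delegate to its UseStarted event.
; The Conversate function, the likely target of that binding, only prints "Hello".
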(event EventBeginPlay
  (bind _asbp_interactable_object (Utilities|Casting|CastToBP_InteractableObject (Variables|/Script/Engine.ChildActorComponent|GetChildActor (Variables|Default|GetConversationInteraction))))
  (EventDispatchers|BindEventtoUseStarted _asbp_interactable_object (EventDispatchers|CreateEvent :!event Conversate)))

(event Collision|EventActorBeginOverlap
  (params (OtherActor :type Actor%20Object%20Reference)))

(event EventTick
  (params (DeltaSeconds :type Float%20%28single-precision%29)))

(fn ConstructionScript
  (Class|SkinnedMeshComponent|SetSkeletalMesh (Variables|Default|GetSkeletalMesh) (Variables|Default|GetCharacterMesh) true)
  (Components|SkeletalMesh|SetAnimInstanceClass (Variables|Default|GetSkeletalMesh) (Variables|Default|GetAnimInstance)))

(fn Conversate
  (Development|PrintString "Hello"))