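; BP_SplinePath is a spline path actor that allowed player types can join from either end.
; Start and end trigger overlaps check the actor's class against UsablePlayerTypes, then look for its SplinePathing component.
; That component receives this path as its new spline, at distance zero or full length respectively, with a debug print.
; The construction script offsets the end trigger by the spline's local end position.
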(event OnComponentBeginOverlap(SplineStartTrigger)
  (params (OverlappedComponent :type Primitive%20Component%20Object%20Reference) (OtherActor :type Actor%20Object%20Reference) (OtherComp :type Primitive%20Component%20Object%20Reference) (OtherBodyIndex :type Integer) (bFromSweep :type Boolean) (SweepResult :type Hit%20Result%20Structure%20%28by%20ref%29))
  (bind _returnvalue (Actor|GetComponentbyClass OtherActor "/Game/Gameplay/Blueprints/Components/SplinePathing.SplinePathing_C"))
  (if (Utilities|Array|ContainsItem (Variables|Default|GetUsablePlayerTypes) (Utilities|GetClass OtherActor))
    (Utilities|IsValid _returnvalue
      (:Is%20Valid
        (Default|SetNewSplinetoFollow _returnvalue self 0.0)
        (Development|PrintString "Spline Start!!")))))

(event OnComponentBeginOverlap(SplineEndTrigger)
  (params (OverlappedComponent :type Primitive%20Component%20Object%20Reference) (OtherActor :type Actor%20Object%20Reference) (OtherComp :type Primitive%20Component%20Object%20Reference) (OtherBodyIndex :type Integer) (bFromSweep :type Boolean) (SweepResult :type Hit%20Result%20Structure%20%28by%20ref%29))
  (bind _returnvalue (Actor|GetComponentbyClass OtherActor "/Game/Gameplay/Blueprints/Components/SplinePathing.SplinePathing_C"))
  (if (Utilities|Array|ContainsItem (Variables|Default|GetUsablePlayerTypes) (Utilities|GetClass OtherActor))
    (Utilities|IsValid _returnvalue
      (:Is%20Valid
        (Default|SetNewSplinetoFollow _returnvalue self (Spline|GetSplineLength (Variables|Default|GetPath)))
        (Development|PrintString "Spline End!!")))))

(event EventBeginPlay)

(event Collision|EventActorBeginOverlap
  (params (OtherActor :type Actor%20Object%20Reference)))

(event EventTick
  (params (DeltaSeconds :type Float%20%28single-precision%29)))

(fn ConstructionScript
  (bind _path (Variables|Default|GetPath))
  (bind _returnvalue (Spline|GetSplineLength _path))
  (bind _returnvalue_2 (Spline|GetLocationatDistanceAlongSpline _path _returnvalue "Local"))
  (Transformation|AddLocalOffset (Variables|Default|GetSplineEndTrigger) (Math|Vector|MakeVector (.x _returnvalue_2) (.y _returnvalue_2) (.z _returnvalue_2)) false false))