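; BP_Haybale_Platform is a hay bale platform that raises and lowers its Hay component on command.
; LiftUP and LiftDown call the GoUp and GoDown events, which play or reverse the HayLifting timeline.
; The timeline's HayLerp track blends the hay's relative transform between its origin and a raised position on Z, without sweeping for collision.
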(event Custom|GoUp
  (bind _haylerp (Timeline|HayLifting Play)
    (:Update
      (Transformation|SetRelativeTransform (Variables|Default|GetHay) (Math|Transform|Lerp(Transform) (Math|Transform|MakeTransform "0, 0, 0" "0.000000, 0, 0") (Math|Transform|MakeTransform "0, 0,100.000000" "0.000000, 0, 0") _haylerp) false false))))

(event Custom|GoDown
  (bind _haylerp (Timeline|HayLifting Reverse)
    (:Update
      (Transformation|SetRelativeTransform (Variables|Default|GetHay) (Math|Transform|Lerp(Transform) (Math|Transform|MakeTransform "0, 0, 0" "0.000000, 0, 0") (Math|Transform|MakeTransform "0, 0,100.000000" "0.000000, 0, 0") _haylerp) false false))))

(event EventBeginPlay)

(event Collision|EventActorBeginOverlap
  (params (OtherActor :type Actor%20Object%20Reference)))

(event EventTick
  (params (DeltaSeconds :type Float%20%28single-precision%29)))

(fn ConstructionScript)

(fn LiftUP
  (CallFunction|GoUp))

(fn LiftDown
  (CallFunction|GoDown))