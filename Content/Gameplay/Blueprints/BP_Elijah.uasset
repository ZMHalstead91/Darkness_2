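; Character Blueprint for Elijah that handles crawling and ladder climbing.
; Crawl, bottom mount and top dismount disable input and play montages, with separate finish events restoring input.
; Ladder mounting switches movement to Flying without orient-to-movement, and dismounting restores Walking, immediately at the bottom or through the finish event at the top.
; An IsClimbing flag gates both dismounts, while the CanJumpInternal override effectively passes through the parent result.
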(event EventDismountLadderTop
  ;[1 1 1] Climbing Stuff
  (CallFunction|LadderDismountTop))

(event EventDismountLadderBottom
  ;[1 1 1] Climbing Stuff
  (CallFunction|LadderDismountBottom))

(event EventFinishCrawling
  (Character|UnCrouch)
  (Input|EnableInput 0))

(event EventMountLadderBottom
  (bind _charactermovement (Variables|Character|GetCharacterMovement))
  ;[1 1 1] Climbing Stuff
  (Input|DisableInput 0)
  (CallFunction|EndInteractState)
  (Pawn|Components|CharacterMovement|SetMovementMode _charactermovement "MOVE_Flying" 0)
  (Variables|/Script/Engine.CharacterMovementComponent|SetbOrientRotationToMovement _charactermovement false)
  (Animation|PlayAnimMontage "/Game/Assets/Elijah/Anims/Elijh_MountLadder_Bottom_Montage.Elijh_MountLadder_Bottom_Montage" 1.0 "None"))

(event EventBeginCrawling
  (Input|DisableInput 0)
  (Character|Crouch)
  (Animation|PlayAnimMontage "/Game/Assets/Elijah/Anims/Elijh_Crawl_Montage.Elijh_Crawl_Montage" 1.0 "None")
  (CallFunction|EndInteractState))

(event EventFinishedMounting
  ;[1 1 1] Climbing Stuff
  (Variables|Default|SetIsClimbing? true)
  (Input|EnableInput 0))

(event EventFinishedDismounting
  (bind _charactermovement (Variables|Character|GetCharacterMovement))
  ;[1 1 1] Climbing Stuff
  (Variables|Default|SetIsClimbing? false)
  (Pawn|Components|CharacterMovement|SetMovementMode _charactermovement "MOVE_Walking" 0)
  (Variables|/Script/Engine.CharacterMovementComponent|SetbOrientRotationToMovement _charactermovement true)
  (Input|EnableInput 0))

(fn ConstructionScript
  (|CallParentFunction))

(fn LadderDismountTop
  (if (Variables|Default|GetIsClimbing?)
    (Variables|Default|SetIsClimbing? false)
    (Input|DisableInput 0)
    (Animation|PlayAnimMontage "/Game/Assets/Elijah/Anims/Elijh_DismountLadder_Top_Montage.Elijh_DismountLadder_Top_Montage" 1.0 "None")))

(fn LadderDismountBottom
  (bind _charactermovement (Variables|Character|GetCharacterMovement))
  (if (Variables|Default|GetIsClimbing?)
    (Variables|Default|SetIsClimbing? false)
    (Pawn|Components|CharacterMovement|SetMovementMode _charactermovement "MOVE_Walking" 0)
    (Variables|/Script/Engine.CharacterMovementComponent|SetbOrientRotationToMovement _charactermovement true)))

(fn CanJumpInternal
  (bind _returnvalue (|CallParentFunction))
  (return (and _returnvalue (not false))))

(fn IsClimbing
  (return (Variables|Default|GetIsClimbing?)))