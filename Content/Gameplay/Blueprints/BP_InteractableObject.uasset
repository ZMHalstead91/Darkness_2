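; Base interactable object, apparently for push-style interactions, that a character can attach to from up to four configurable sides.
; The construction script sizes mesh, collision and triggers, which register the object and side with overlapping characters.
; BeginUse attaches the player at that side's offset, and Tick interpolates their facing and optional position.
; MoveForward filters input through auto-release, allowed-direction and sphere-trace checks, storing it without moving the object.
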(event OnComponentBeginOverlap(TriggerA)
  (params (OverlappedComponent :type Primitive%20Component%20Object%20Reference) (OtherActor :type Actor%20Object%20Reference) (OtherComp :type Primitive%20Component%20Object%20Reference) (OtherBodyIndex :type Integer) (bFromSweep :type Boolean) (SweepResult :type Hit%20Result%20Structure%20%28by%20ref%29))
  (CallFunction|BeginTriggerOverlap OtherActor (Variables|Default|GetInteractionSideA) (Variables|Default|GetTriggerA)))

(event OnComponentEndOverlap(TriggerA)
  (params (OverlappedComponent :type Primitive%20Component%20Object%20Reference) (OtherActor :type Actor%20Object%20Reference) (OtherComp :type Primitive%20Component%20Object%20Reference) (OtherBodyIndex :type Integer))
  (CallFunction|EndTriggerOverlap OtherActor (Variables|Default|GetInteractionSideA) (Variables|Default|GetTriggerA)))

(event OnComponentBeginOverlap(TriggerB)
  (params (OverlappedComponent :type Primitive%20Component%20Object%20Reference) (OtherActor :type Actor%20Object%20Reference) (OtherComp :type Primitive%20Component%20Object%20Reference) (OtherBodyIndex :type Integer) (bFromSweep :type Boolean) (SweepResult :type Hit%20Result%20Structure%20%28by%20ref%29))
  (CallFunction|BeginTriggerOverlap OtherActor (Variables|Default|GetInteractionSideB) (Variables|Default|GetTriggerB)))

(event OnComponentEndOverlap(TriggerB)
  (params (OverlappedComponent :type Primitive%20Component%20Object%20Reference) (OtherActor :type Actor%20Object%20Reference) (OtherComp :type Primitive%20Component%20Object%20Reference) (OtherBodyIndex :type Integer))
  (CallFunction|EndTriggerOverlap OtherActor (Variables|Default|GetInteractionSideB) (Variables|Default|GetTriggerB)))

(event OnComponentBeginOverlap(TriggerC)
  (params (OverlappedComponent :type Primitive%20Component%20Object%20Reference) (OtherActor :type Actor%20Object%20Reference) (OtherComp :type Primitive%20Component%20Object%20Reference) (OtherBodyIndex :type Integer) (bFromSweep :type Boolean) (SweepResult :type Hit%20Result%20Structure%20%28by%20ref%29))
  (CallFunction|BeginTriggerOverlap OtherActor (Variables|Default|GetInteractionSideC) (Variables|Default|GetTriggerC)))

(event OnComponentEndOverlap(TriggerC)
  (params (OverlappedComponent :type Primitive%20Component%20Object%20Reference) (OtherActor :type Actor%20Object%20Reference) (OtherComp :type Primitive%20Component%20Object%20Reference) (OtherBodyIndex :type Integer))
  (CallFunction|EndTriggerOverlap OtherActor (Variables|Default|GetInteractionSideC) (Variables|Default|GetTriggerC)))

(event OnComponentBeginOverlap(TriggerD)
  (params (OverlappedComponent :type Primitive%20Component%20Object%20Reference) (OtherActor :type Actor%20Object%20Reference) (OtherComp :type Primitive%20Component%20Object%20Reference) (OtherBodyIndex :type Integer) (bFromSweep :type Boolean) (SweepResult :type Hit%20Result%20Structure%20%28by%20ref%29))
  (CallFunction|BeginTriggerOverlap OtherActor (Variables|Default|GetInteractionSideD) (Variables|Default|GetTriggerD)))

(event OnComponentEndOverlap(TriggerD)
  (params (OverlappedComponent :type Primitive%20Component%20Object%20Reference) (OtherActor :type Actor%20Object%20Reference) (OtherComp :type Primitive%20Component%20Object%20Reference) (OtherBodyIndex :type Integer))
  (CallFunction|EndTriggerOverlap OtherActor (Variables|Default|GetInteractionSideD) (Variables|Default|GetTriggerD)))

(event EventBeginPlay)

(event Collision|EventActorBeginOverlap
  (params (OtherActor :type Actor%20Object%20Reference)))

(event EventTick
  (params (DeltaSeconds :type Float%20%28single-precision%29))
  (CallFunction|UpdateInteractionActor DeltaSeconds))

(fn ConstructionScript
  (CallFunction|SetupObjMesh)
  (CallFunction|SetCollisionExtents)
  (Interaction|SetupTriggers))

(fn SetupTriggers
  (Utilities|FlowControl|Sequence
    (:then_0
      (Interaction|SetTriggerActive (Variables|Default|GetTriggerA) (Variables|Default|GetInteractionSideA)))
    (:then_1
      (Interaction|SetTriggerActive (Variables|Default|GetTriggerB) (Variables|Default|GetInteractionSideB)))
    (:then_2
      (Interaction|SetTriggerActive (Variables|Default|GetTriggerC) (Variables|Default|GetInteractionSideC)))
    (:then_3
      (Interaction|SetTriggerActive (Variables|Default|GetTriggerD) (Variables|Default|GetInteractionSideD)))))

(fn SetTriggerActive
  (params (BoxTrigger :type Box%20Component%20Object%20Reference) (InteractionOptions :type Struct%20Interaction%20Options%20Structure))
  (bind (_bactive _bforward _bbackward _bright _bleft _direction) (Utilities|Struct|BreakStruct_InteractionOptions InteractionOptions))
  (bind _output_get (LocalVariables|SetTriggerUpdate BoxTrigger))
  (Rendering|SetVisibility _output_get _bactive false)
  (Collision|SetCollisionEnabled (LocalVariables|GetTriggerUpdate) (select _bactive "QueryOnly" "NoCollision"))
  (bind _output_get_2 (LocalVariables|SetTriggerDirection _direction))
  (Transformation|SetRelativeRotation (LocalVariables|GetTriggerUpdate) (Math|Rotator|MakeRotfromX _output_get_2) false false)
  (Components|Box|SetBoxExtent (LocalVariables|GetTriggerUpdate) (Utilities|GetTriggerExtents) false)
  (Transformation|SetRelativeLocation (LocalVariables|GetTriggerUpdate) (Utilities|GetTriggerRelativeLocation (LocalVariables|GetTriggerDirection)) false false))

(fn SetupObjMesh
  (Components|StaticMesh|SetStaticMesh (Variables|Default|GetMesh) (Variables|Default|GetObjMesh))
  (Transformation|SetWorldScale3D (Variables|Default|GetMesh) (Math|Vector|SelectVector (Variables|Default|GetCustomMeshScale) (Variables|Default|GetObjScale) (Variables|Default|GetbCustomMeshScale)))
  (Transformation|SetRelativeLocation (Variables|Default|GetMesh) (Variables|Default|GetMeshOffset) false false)
  (return))

(fn SetCollisionExtents
  (Components|Box|SetBoxExtent (Variables|Default|GetMeshCollision) (- (* (Variables|Default|GetObjScale) (Variables|Default|GetDefaultBoxExtents)) (Variables|Default|GetCollisionExtentOffset)) false))

(fn BeginUse
  (params (Character :type Character%20Object%20Reference) (InteractSide :type Struct%20Interaction%20Options%20Structure) (Trigger :type Box%20Component%20Object%20Reference))
  (CallFunction|ActivateInteractSide Character InteractSide Trigger)
  (bind _interactingplayer (Variables|Default|GetInteractingPlayer)
    (:then
      (Transformation|AttachComponentToComponent _interactingplayer (Variables|Default|GetPlayerLocation) "None" "KeepWorld" "KeepWorld" "KeepWorld" true)
      (Default|CallUseStarted)
      (return true))
    (:else
      (return false))))

(fn EndUse
  (bind _interactingplayer (Variables|Default|GetInteractingPlayer)
    (:then
      (Transformation|DetachFromActor _interactingplayer "KeepWorld" "KeepWorld" "KeepWorld")
      (Variables|Default|SetInteractingPlayer 0)
      (Variables|Default|SetInteractingController 0)
      (Default|CallUseEnded))
    (:else)))

(fn MoveForward
  (params (InputPin :type Float%20%28single-precision%29))
  (LocalVariables|SetInput InputPin)
  (bind _direction (CallFunction|GetMoveDirection true))
  (LocalVariables|SetDirection _direction)
  (bind _notreleased (CallFunction|CheckAutoRelease (* (LocalVariables|GetDirection) (LocalVariables|GetInput))))
  (if _notreleased
    (bind _bcanmove (CallFunction|CanMoveinDirection true (* (LocalVariables|GetDirection) (LocalVariables|GetInput)) (LocalVariables|GetInput)))
    (if _bcanmove
      (bind _canmove (CallFunction|CheckCharacterMovement (* (LocalVariables|GetDirection) (LocalVariables|GetInput))))
      (if _canmove
        (bind _output_get (Variables|Default|SetInputForward (LocalVariables|GetInput)))
        (else
          (Variables|Default|SetInputForward 0.0 :!label _label)))
      (else
        (goto _label)))
    (else
      (goto _label))))

(fn BeginTriggerOverlap
  (params (Actor :type Actor%20Object%20Reference) (SideOptions :type Struct%20Interaction%20Options%20Structure) (Trigger :type Box%20Component%20Object%20Reference))
  (bind _ascharacter (Utilities|Casting|CastToCharacter Actor))
  (Class|BPIObjectInteraction|AddUsableActor(Message) _ascharacter (Utilities|Struct|MakeStruct_InteractableActor self SideOptions Trigger)))

(fn EndTriggerOverlap
  (params (Actor :type Actor%20Object%20Reference) (SideOptions :type Struct%20Interaction%20Options%20Structure) (Trigger :type Box%20Component%20Object%20Reference))
  (bind _ascharacter (Utilities|Casting|CastToCharacter Actor))
  (Class|BPIObjectInteraction|RemoveUsableActor(Message) _ascharacter (Utilities|Struct|MakeStruct_InteractableActor self SideOptions Trigger)))

(fn ActivateInteractSide
  (params (Character :type Character%20Object%20Reference) (PushSide :type Struct%20Interaction%20Options%20Structure) (Trigger :type Box%20Component%20Object%20Reference))
  (CallFunction|SetPlayerCharacter Character)
  (bind _output_get (Variables|Default|SetInteractSideCurrent PushSide))
  (Variables|Default|SetTriggerCurrent Trigger)
  (bind _output_get_2 (Variables|Default|SetForwardDirection (* (Math|Transform|TransformDirection (Transformation|GetActorTransform) (.Direction (Utilities|Struct|BreakStruct_InteractionOptions _output_get))) -1.0)))
  (Variables|Default|SetRightDirection (* (Math|Vector|CrossProduct _output_get_2 "0, 0,1.000000") -1.0))
  (Transformation|SetRelativeLocationAndRotation (Variables|Default|GetPlayerLocation) (* (+ (* (Variables|Default|GetObjScale) (Variables|Default|GetDefaultBoxExtents)) (Variables|Default|GetCharacterInteractOffset)) (.Direction (Utilities|Struct|BreakStruct_InteractionOptions (Variables|Default|GetInteractSideCurrent)))) (Math|Rotator|MakeRotfromX (.Direction (Utilities|Struct|BreakStruct_InteractionOptions (Variables|Default|GetInteractSideCurrent)))) false false) ; Set offset location to use for later
)

(fn SetPlayerCharacter
  (params (PlayerCharacter :type Character%20Object%20Reference))
  (bind _output_get (Variables|Default|SetInteractingPlayer PlayerCharacter))
  (Utilities|IsValid _output_get
    (:Is%20Valid
      (bind _asplayer_controller (Utilities|Casting|CastToPlayerController (Pawn|GetController _output_get)))
      (Variables|Default|SetInteractingController _asplayer_controller))))

(fn MoveUp
  (params (InputPin :type Float%20%28single-precision%29)))

(fn UpdateInteractionActor
  (params (DeltaTime :type Float%20%28single-precision%29))
  (Variables|Default|SetDeltaTime DeltaTime)
  (CallFunction|CharacterFaceInteraction)
  (CallFunction|UpdateCharacterOffset))

(fn CharacterFaceInteraction
  (bind _forwarddirection (Variables|Default|GetForwardDirection))
  (bind _returnvalue (Math|Rotator|MakeRotfromX _forwarddirection))
  (bind _interactingplayer (Variables|Default|GetInteractingPlayer) ; Only if we have a push character
    (:then
      (if (Utilities|Enum|NotEqual(Enum) _returnvalue (Transformation|GetActorRotation _interactingplayer) 0.5) ; Only update if we are not within 0.5 of the rotation
        (Transformation|SetActorRotation (Variables|Default|GetInteractingPlayer) (Math|Interpolation|RInterpTo (Transformation|GetActorRotation (Variables|Default|GetInteractingPlayer)) (Math|Rotator|MakeRotator 0.0 0.0 (.Yaw (Math|Rotator|BreakRotator _returnvalue))) (Variables|Default|GetDeltaTime) (/ (.Yaw (Math|Rotator|BreakRotator (Variables|/Script/Engine.CharacterMovementComponent|GetRotationRate (Variables|/Script/Engine.Character|GetCharacterMovement _interactingplayer)))) 9e+01))) ; Set character to face push over time
      ))
    (:else)))

(fn UpdateCharacterOffset
  (bind _playerlocation (Variables|Default|GetPlayerLocation))
  (bind _returnvalue (Transformation|GetWorldLocation _playerlocation))
  (if (Variables|Default|GetbUpdateOffset) ; Only update if we set true
    (bind _interactingplayer (Variables|Default|GetInteractingPlayer) ; Only update if we have a character
      (:then
        (Transformation|SetActorLocation _interactingplayer (Math|Interpolation|VInterpTo (Transformation|GetActorLocation (Variables|Default|GetInteractingPlayer)) (Math|Vector|MakeVector (.x _returnvalue) (.y _returnvalue) (.z (Transformation|GetActorLocation (Variables|Default|GetInteractingPlayer)))) (Variables|Default|GetDeltaTime) 6.0) true false) ; Move the character to the correct offset position
      )
      (:else))))

(fn CheckAutoRelease
  (params (Direction :type Vector))
  (if (Variables|Default|GetbAutoRelease)
    (bind _interactingplayer (Variables|Default|GetInteractingPlayer)
      (:then
        (if (<= (Math|Vector|DotProduct Direction (Transformation|GetActorForwardVector _interactingplayer)) -0.75)
          (bind _interactingplayer_2 (Variables|Default|GetInteractingPlayer)
            (:then
              (Class|BPIObjectInteraction|ToggleInteract(Message) _interactingplayer_2 false 0.0))
            (:else
              _))
          (LocalVariables|SetNoPushRelease false)
          (else
            (LocalVariables|SetNoPushRelease true :!label _label))))
      (:else
        (goto _label)))
    (else
      (goto _label)))
  (return (LocalVariables|GetNoPushRelease)))

(fn GetMoveDirection
  (params (Forward :type Boolean))
  (LocalVariables|SetForward%20Direction Forward)
  (return (Math|Vector|SelectVector (Variables|Default|GetForwardDirection) (Variables|Default|GetRightDirection) (LocalVariables|GetForward%20Direction))))

(fn CanMoveinDirection
  (params (Forward :type Boolean) (Direction :type Vector) (Input :type Float%20%28single-precision%29))
  (bind _interactsidecurrent (Variables|Default|GetInteractSideCurrent))
  (bind (_bactive _bforward _bbackward _bright _bleft) (Utilities|Struct|BreakStruct_InteractionOptions _interactsidecurrent))
  (LocalVariables|SetbForwardDirection Forward)
  (LocalVariables|SetMovementDirection Direction)
  (return (and (select (< Input 0.0) (select (LocalVariables|GetbForwardDirection) _bbackward _bleft) (select (LocalVariables|GetbForwardDirection) _bforward _bright)) (or (not (Variables|Default|GetbSingleDirection)) (== (Math|Float|SelectFloat (Variables|Default|GetInputRight) (Variables|Default|GetInputForward) (LocalVariables|GetbForwardDirection)) 0.0)))))

(fn CheckCharacterMovement
  (params (Direction :type Vector))
  (bind _returnvalue (Transformation|GetVelocity))
  (bind _interactingplayer (Variables|Default|GetInteractingPlayer))
  (bind _returnvalue_2 (Math|Vector|Normalize _returnvalue))
  (bind _returnvalue_3 (Transformation|GetActorLocation _interactingplayer))
  (bind (_x _y) (Math|Vector|BreakVector _returnvalue_2))
  (LocalVariables|SetDir Direction)
  (bind _interactingplayer_2 (Variables|Default|GetInteractingPlayer)
    (:then
      (LocalVariables|SetRadius (Components|Capsule|GetScaledCapsuleRadius (Variables|/Script/Engine.Character|GetCapsuleComponent _interactingplayer_2)))
      (if (Math|Vector|Equal(Vector) (Math|Vector|SelectVector (Math|Vector|MakeVector _x _y 0.0) (LocalVariables|GetDir) (!= (Math|Vector|VectorLength (LocalVariables|GetDir)) 0.0)) "0, 0, 0" 0.0001)
        _
        (else
          (bind _returnvalue_4 (Collision|SphereTraceByChannel _returnvalue_3 (+ _returnvalue_3 (* (Math|Vector|SelectVector (Math|Vector|MakeVector _x _y 0.0) (LocalVariables|GetDir) (!= (Math|Vector|VectorLength (LocalVariables|GetDir)) 0.0)) (LocalVariables|GetRadius))) (LocalVariables|GetRadius) "TraceTypeQuery1" false (Utilities|Array|MakeArray (Variables|Default|GetInteractingPlayer)) "None"))
          (if _returnvalue_4
            _
            (else
              _)))))
    (:else
      _))
  (return (not _returnvalue_4)))

(fn PostObjectUsed)