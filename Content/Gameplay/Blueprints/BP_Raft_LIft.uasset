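; BP_Raft_LIft is a lift actor that pairs a child BP_Raft with a child lever that triggers its movement.
; On BeginPlay it copies its GoUP setting to the raft and binds MovePlatform to the lever's use-started event.
; MovePlatform calls the raft's GoUp regardless of lever toggle state, then plays a rope-tightening 2D sound at the game instance's effects volume.
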(event Custom|Move%20Platform
  (bind _asbp_raft (Utilities|Casting|CastToBP_Raft (Variables|/Script/Engine.ChildActorComponent|GetChildActor (Variables|Default|GetBP_Raft))))
  (if (Variables|/Game/BP_InteractiveObject_Lever.BP_InteractiveObject_Lever_C|GetToggle (stale EventBeginPlay _asbp_interactive_object_lever))
    _
    (else
      _))
  (Default|GoUp _asbp_raft)
  (bind _asbp_darkness_game_instance (Utilities|Casting|CastToBP_Darkness_GameInstance (Game|GetGameInstance)))
  (Audio|SpawnSound2D "/Game/Audio/Rope_Tighten_Long.Rope_Tighten_Long" (Variables|/Game/Base/BP_Darkness_GameInstance.BP_Darkness_GameInstance_C|GetEffectsVolume _asbp_darkness_game_instance)))

(event EventBeginPlay
  (bind _asbp_raft (Utilities|Casting|CastToBP_Raft (Variables|/Script/Engine.ChildActorComponent|GetChildActor (Variables|Default|GetBP_Raft))))
  (Variables|/Game/Gameplay/Blueprints/BP_Raft.BP_Raft_C|SetGO%20UP _asbp_raft (Variables|Default|GetGo%20UP))
  (bind _asbp_interactive_object_lever (Utilities|Casting|CastToBP_InteractiveObject_Lever (Variables|/Script/Engine.ChildActorComponent|GetChildActor (Variables|Default|GetBP_InteractiveObject_Lever))))
  (EventDispatchers|BindEventtoUseStarted _asbp_interactive_object_lever (delegate Custom|Move%20Platform)))

(event Collision|EventActorBeginOverlap
  (params (OtherActor :type Actor%20Object%20Reference)))

(event EventTick
  (params (DeltaSeconds :type Float%20%28single-precision%29)))

(fn ConstructionScript)