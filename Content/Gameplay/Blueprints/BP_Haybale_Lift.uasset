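; BP_Haybale_Lift is a lever-operated lift that raises and lowers a haybale platform.
; It assembles a lever and a platform as child actors.
; On BeginPlay it binds MovePlatform to the lever's use-started event.
; MovePlatform reads the lever's toggle state and calls GoDown on the platform when it is set, GoUp otherwise.
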(event Custom|Move%20Platform
  (bind _asbp_haybale_platform (Utilities|Casting|CastToBP_Haybale_Platform (Variables|/Script/Engine.ChildActorComponent|GetChildActor (Variables|Default|GetBP_Haybale_Platform))))
  (if (Variables|/Game/BP_InteractiveObject_Lever.BP_InteractiveObject_Lever_C|GetToggle (stale EventBeginPlay _asbp_interactive_object_lever))
    (Default|GoDown _asbp_haybale_platform)
    (else
      (Default|GoUp _asbp_haybale_platform))))

(event EventBeginPlay
  (bind _asbp_interactive_object_lever (Utilities|Casting|CastToBP_InteractiveObject_Lever (Variables|/Script/Engine.ChildActorComponent|GetChildActor (Variables|Default|GetBP_InteractiveObject_Lever))))
  (EventDispatchers|BindEventtoUseStarted _asbp_interactive_object_lever (delegate Custom|Move%20Platform)))

(event Collision|EventActorBeginOverlap
  (params (OtherActor :type Actor%20Object%20Reference)))

(event EventTick
  (params (DeltaSeconds :type Float%20%28single-precision%29)))

(fn ConstructionScript)