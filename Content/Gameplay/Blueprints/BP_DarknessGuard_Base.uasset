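; Base guard NPC that raises an alert while it detects the player and triggers game over when that alert fills.
; PlayerDetected/PlayerLost toggle PlayerFound, driving an alert sound and a per-tick investigate meter, not delta-time scaled, on a camera-facing widget.
; An optional lantern, lit according to ViewRange, follows the hand socket each tick instead of being attached.
; Whip spawning is stubbed out, and SpawnPatrolPoints is not called here.
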(event EventBeginPlay
  (|CallParentFunction)
  (CallFunction|TrySpawnLanternAttached)
  (CallFunction|TrySpawnWhipAttached))

(event Collision|EventActorBeginOverlap
  (params (OtherActor :type Actor%20Object%20Reference)))

(event EventPlayerDetected
  (bind _output_get (Variables|Investigation|SetPlayerFound? true))
  (Utilities|FlowControl|DoOnce false
    (:Completed
      (Rendering|SetVisibility (Variables|Default|GetInvestigateWidget) _output_get false))))

(event EventPlayerLost
  (Variables|Investigation|SetPlayerFound? false)
  (Utilities|FlowControl|DoOnce false) ; enters at Reset
)

(event EventTick
  (params (DeltaSeconds :type Float%20%28single-precision%29))
  (bind _mesh (Variables|Character|GetMesh))
  (bind _rpalmsocketname (Variables|Default|GetRPalmSocketName))
  (bind _returnvalue (Transformation|GetSocketTransform _mesh _rpalmsocketname "RTS_World"))
  (Transformation|SetActorLocationAndRotation (Variables|Default|GetLantern) (.location _returnvalue) (Math|Rotator|MakeRotator 0.0 0.0 (.yaw (.rotation _returnvalue))))
  (Variables|/Script/Engine.CharacterMovementComponent|SetMaxWalkSpeed (Variables|Character|GetCharacterMovement) (* (Variables|Default|GetSpeedRate) (Variables|Default|GetSpeedVariable)))
  (Investigation|UpdateInvestigateProgress)
  (Investigation|DisplayInvestigateProgress)
  (Investigation|GameOverCheck)
  (if (Variables|Investigation|GetPlayerFound?)
    (Utilities|FlowControl|DoOnce false :!label _label
      (:Completed
        (Audio|PlaySoundatLocation "/Game/Audio/Alert_Cue.Alert_Cue" (Transformation|GetActorLocation) "0, 0, 0" 4.0)))
    (else
      (goto _label Reset))))

(fn ConstructionScript
  (|CallParentFunction))

(fn TrySpawnLanternAttached
  (bind _viewrange (Variables|Default|GetViewRange))
  (if (Variables|Default|GetShouldHaveLantern?)
    (bind _returnvalue (Game|SpawnActorfromClass "/Game/Gameplay/Blueprints/Lantern.Lantern_C" (Math|Transform|MakeTransform "0, 0, 0") "AlwaysSpawn" 0 0))
    (Variables|Default|SetLantern _returnvalue)
    (Rendering|Lighting|SetAttenuationRadius (Variables|/Game/Gameplay/Blueprints/Lantern.Lantern_C|GetPointLight _returnvalue) (* _viewrange 1.25))
    (Class|PointLightComponent|SetSourceRadius (Variables|/Game/Gameplay/Blueprints/Lantern.Lantern_C|GetPointLight _returnvalue) _viewrange))
  (bind _asanim_bp_male_npc (Utilities|Casting|CastToAnimBP_MaleNPC (Components|SkeletalMesh|GetAnimInstance (Variables|Character|GetMesh))))
  (Variables|/Game/Assets/MaleNPC/Anims/AnimBP_MaleNPC.AnimBP_MaleNPC_C|SetHasLantern? _asanim_bp_male_npc (Variables|Default|GetShouldHaveLantern?)))

(fn TrySpawnWhipAttached
  (if (Variables|Default|GetShouldHaveWhip?)
    _))

(fn SpawnPatrolPoints
  (bind _self self)
  (bind _self_2 self)
  (Game|SpawnActorfromClass "/Game/Gameplay/Blueprints/AI/BP_BotWaypoint.BP_BotWaypoint_C" (Transformation|GetWorldTransform (Variables|Default|GetPatrolPoint_00)) "AlwaysSpawn" _self 0 _self)
  (Game|SpawnActorfromClass "/Game/Gameplay/Blueprints/AI/BP_BotWaypoint.BP_BotWaypoint_C" (Transformation|GetWorldTransform (Variables|Default|GetPatrolPoint_01)) "AlwaysSpawn" _self_2 1 _self_2))

(fn UpdateInvestigateProgress
  (if (Variables|Investigation|GetPlayerFound?)
    (Variables|Investigation|SetInvestigateProgress (Math|Float|Clamp(Float) (+ (Variables|Investigation|GetInvestigateProgress) (Variables|Investigation|GetIvestigateIncrement)) 0.0 1.0))
    (else
      (Variables|Investigation|SetInvestigateProgress (Math|Float|Clamp(Float) (- (Variables|Investigation|GetInvestigateProgress) (Variables|Investigation|GetIvestigateIncrement)) 0.0 1.0)))))

(fn DisplayInvestigateProgress
  (bind _returnvalue (Game|GetPlayerCameraManager 0))
  (bind _investigatescene (Variables|Default|GetInvestigateScene))
  (bind _investigateprogress (Variables|Investigation|GetInvestigateProgress))
  (bind _returnvalue_2 (Transformation|GetWorldLocation _investigatescene))
  (bind _returnvalue_3 (Camera|GetCameraLocation _returnvalue))
  (bind _returnvalue_4 (Math|Rotator|FindLookatRotation _returnvalue_2 _returnvalue_3))
  (bind (_roll _pitch _yaw) (Math|Rotator|BreakRotator _returnvalue_4))
  (bind _asw_investigate_behavior (Utilities|Casting|CastToW_InvestigateBehavior (UserInterface|GetUserWidgetObject (Variables|Default|GetInvestigateWidget))))
  (Default|SetAlertProgress _asw_investigate_behavior _investigateprogress)
  (if (> _investigateprogress 0.0)
    (Transformation|SetWorldRotation _investigatescene _returnvalue_4 false false)
    (Transformation|SetWorldRotation _investigatescene (Math|Rotator|MakeRotator _roll 0.0 _yaw) false false)
    (else
      (Rendering|SetVisibility (Variables|Default|GetInvestigateWidget) false false))))

(fn GameOverCheck
  (if (>= (Variables|Investigation|GetInvestigateProgress) 1.0)
    (bind _asgm_gameplay_base (Utilities|Casting|CastToGM_GameplayBase (Game|GetGameMode)))
    (Default|GameOver _asgm_gameplay_base)))