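; BP_Pickup is a usable pickup actor that announces its ObjectID when used, then destroys itself.
; At BeginPlay it caches every actor implementing ItemPickupInterface as its listeners, so the Used event can send each one ItemPickedUpMessage.
; CanUse and ShouldAutoRemove both return false here.
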(event EventBeginPlay
  (bind _outactors (Actor|GetAllActorswithInterface "/Game/Gameplay/Blueprints/Interfaces/ItemPickupInterface.ItemPickupInterface_C"))
  (Variables|Default|SetPickupListeners _outactors))

(event Collision|EventActorBeginOverlap
  (params (OtherActor :type Actor%20Object%20Reference)))

(event EventTick
  (params (DeltaSeconds :type Float%20%28single-precision%29)))

(event EventUsed
  (params (UsingActor :type Actor%20Object%20Reference) (Value :type Integer))
  (for _array_element (Variables|Default|GetPickupListeners)
    (Class|ItemPickupInterface|ItemPickedUp(Message) _array_element (Variables|Default|GetObjectID)))
  (Actor|DestroyActor))

(fn ConstructionScript)

(fn CanUse?
  (params (UsingActor :type Actor%20Object%20Reference))
  (return false))

(fn ShouldAutoRemove?
  (return false))