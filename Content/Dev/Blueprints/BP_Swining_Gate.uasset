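; A swinging gate that opens on its own once it is unlocked.
; Each Tick while unlocked, RotatePoint yaws one degree until it reaches 90, so opening speed depends on frame rate.
; Unlock writes the Locked flag from its input and, when that is false, disables collision on Cube, with no path to restore it.
; CanUse and ShouldAutoRemove both return false.
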(event EventBeginPlay)

(event Collision|EventActorBeginOverlap
  (params (OtherActor :type Actor%20Object%20Reference)))

(event EventTick
  (params (DeltaSeconds :type Float%20%28single-precision%29))
  (if (not (Variables|Default|GetLocked))
    (if (not (>= (.Yaw (Math|Rotator|BreakRotator (.Rotation (Math|Transform|BreakTransform (Transformation|GetRelativeTransform (Variables|Default|GetRotatePoint)))))) 9e+01))
      (Transformation|AddLocalRotation (Variables|Default|GetRotatePoint) "0,1.000000, 0" false false))))

(fn ConstructionScript)

(fn Unlock
  (params (Locked? :type Boolean))
  (if Locked?
    (Variables|Default|SetLocked Locked?)
    (else
      (Collision|SetCollisionEnabled (Variables|Default|GetCube) "NoCollision")
      (Variables|Default|SetLocked Locked?))))

(fn CanUse?
  (params (UsingActor :type Actor%20Object%20Reference))
  (return false))

(fn ShouldAutoRemove?
  (return false))