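; Game mode for the Grace and Elijah character pair, letting the player swap between them while AI controls the other.
; On start it finds both placed actors and runs a spline-follow behavior tree on Elijah targeting Grace.
; Switching exchanges possession, retargets the blackboard, preserves the follow state and animates the portrait widget if valid.
; Player-start spawning and portrait widget setup exist but are disconnected.
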(event Custom|SetShouldFollow
  (params (ShouldFollow? :type Boolean))
  (bind _aicon_ref (Variables|Default|GetAICon_Ref))
  (Utilities|IsValid _aicon_ref
    (:Is%20Valid
      (bind _asbp_player_base (Utilities|Casting|CastToBP_PlayerBase (Pawn|GetControlledPawn _aicon_ref)))
      (bind _output_get (Variables|/Game/Base/BP_PlayerBase.BP_PlayerBase_C|SetFollowing? _asbp_player_base ShouldFollow?))
      (AI|Components|Blackboard|SetValueasBool (AI|GetBlackboard _aicon_ref) (Variables|Default|GetFollowKeyName) _output_get)
      (Variables|Default|SetTogether? _output_get))))

(event Custom|Initialize
  (bind _asaicontroller (Utilities|Casting|CastToAIController (Pawn|GetController (Variables|Default|GetElijahRef))))
  (bind _output_get (Variables|Default|SetAICon_Ref _asaicontroller))
  (AI|RunBehaviorTree _output_get "/Game/Gameplay/Blueprints/AI/BT_PlayerSplineFollow.BT_PlayerSplineFollow")
  (AI|Components|Blackboard|SetValueasObject (AI|GetBlackboard _output_get) (Variables|Default|GetActorToFollowKeyName) (Variables|Default|GetGraceRef))
  (CallFunction|SetShouldFollow true))

(event EventTick
  (params (DeltaSeconds :type Float%20%28single-precision%29)))

(event EventToggleShouldFollow
  (bind _aicon_ref (Variables|Default|GetAICon_Ref))
  (Utilities|IsValid _aicon_ref
    (:Is%20Valid
      (bind _asbp_player_base (Utilities|Casting|CastToBP_PlayerBase (Pawn|GetControlledPawn _aicon_ref)))
      (bind _output_get (Variables|/Game/Base/BP_PlayerBase.BP_PlayerBase_C|SetFollowing? _asbp_player_base (not (Variables|/Game/Base/BP_PlayerBase.BP_PlayerBase_C|GetFollowing? _asbp_player_base))))
      (AI|Components|Blackboard|SetValueasBool (AI|GetBlackboard _aicon_ref) (Variables|Default|GetFollowKeyName) _output_get)
      (Variables|Default|SetTogether? _output_get))))

(event EventHidePlayerCharacters
  (Input|DisableInput (Variables|Default|GetGraceRef) 0)
  (Actor|DestroyActor (Variables|Default|GetGraceRef))
  (Variables|Default|SetGraceRef 0)
  (Actor|DestroyActor (Variables|Default|GetElijahRef))
  (Variables|Default|SetElijahRef 0))

(event EventSwitchCharacter
  (bind _aicon_ref (Variables|Default|GetAICon_Ref))
  (bind _elijahref (Variables|Default|GetElijahRef))
  (bind _graceref (Variables|Default|GetGraceRef))
  (bind _aicon_ref_2 (Variables|Default|GetAICon_Ref))
  (bind _playerswitchwidg_ref (Variables|Default|GetPlayerSwitchWidg_Ref))
  (bind _switchtograce (Variables|/Game/UI/W_Portraits.W_Portraits_C|GetSwitchToGrace _playerswitchwidg_ref))
  (Character|Crouch (Game|GetPlayerCharacter 0))
  (if (== (Game|Player|GetPlayerPawn 0) (Variables|Default|GetGraceRef))
    (Pawn|Possess (Game|GetPlayerController 0) _elijahref)
    (Pawn|Possess _aicon_ref (Variables|Default|GetGraceRef))
    (AI|RunBehaviorTree _aicon_ref "/Game/Gameplay/Blueprints/AI/BT_PlayerSplineFollow.BT_PlayerSplineFollow")
    (AI|Components|Blackboard|SetValueasObject (AI|GetBlackboard _aicon_ref) (Variables|Default|GetActorToFollowKeyName) _elijahref)
    (Utilities|IsValid _playerswitchwidg_ref
      (:Is%20Valid
        (UserInterface|Animation|PlayAnimation _playerswitchwidg_ref _switchtograce 0.0 1 "Reverse" 1.0))
      (:Is%20Not%20Valid
        _))
    (else
      (Pawn|Possess (Game|GetPlayerController 0) _graceref)
      (Pawn|Possess _aicon_ref_2 (Variables|Default|GetElijahRef))
      (AI|RunBehaviorTree _aicon_ref_2 "/Game/Gameplay/Blueprints/AI/BT_PlayerSplineFollow.BT_PlayerSplineFollow")
      (AI|Components|Blackboard|SetValueasObject (AI|GetBlackboard _aicon_ref_2) (Variables|Default|GetActorToFollowKeyName) _graceref)
      (Utilities|IsValid _playerswitchwidg_ref
        (:Is%20Valid
          (UserInterface|Animation|PlayAnimation _playerswitchwidg_ref _switchtograce 0.0 1 "Forward" 1.0))
        (:Is%20Not%20Valid
          _))))
  (CallFunction|SetShouldFollow (Variables|Default|GetTogether?)))

(event EventBeginPlay
  (bind _outactors (Actor|GetAllActorsOfClass "/Game/Gameplay/Blueprints/BP_Grace.BP_Grace_C"))
  (Variables|Default|SetGraceRef (Utilities|Array|Get(acopy) _outactors))
  (bind _outactors_2 (Actor|GetAllActorsOfClass "/Game/Gameplay/Blueprints/BP_Elijah.BP_Elijah_C"))
  (Variables|Default|SetElijahRef (Utilities|Array|Get(acopy) _outactors_2))
  (Utilities|FlowControl|Delay 0.2)
  (CallFunction|Initialize))

(fn ConstructionScript
  (|CallParentFunction))